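; BP_Note is a readable note pickup that the player can open when standing near it.
; Overlapping its box toggles CanTakeNote on the ThirdPersonQuentin character.
; ReadNote creates the Note widget, sets its image brush from the Note variable and plays an opening sound.
; Stopreading calls ReadingStop on the widget, removes it and plays a closing sound.
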(event `self.Box.OnComponentBeginOverlap`
  (params (OverlappedComponent :type "PrimitiveComponent Object Reference") (OtherActor :type "Actor Object Reference") (OtherComp :type "PrimitiveComponent Object Reference") (OtherBodyIndex :type Integer) (bFromSweep :type Boolean) (SweepResult :type "HitResult Structure (by ref)"))
  (bind _asthird_person_quentin (cast `/Game/AjoutsQuentin/ThirdPersonQuentin` OtherActor))
  (set `/Game/AjoutsQuentin/ThirdPersonQuentin.CanTakeNote` true _asthird_person_quentin))

(event `self.Box.OnComponentEndOverlap`
  (params (OverlappedComponent :type "PrimitiveComponent Object Reference") (OtherActor :type "Actor Object Reference") (OtherComp :type "PrimitiveComponent Object Reference") (OtherBodyIndex :type Integer))
  (bind _asthird_person_quentin (cast `/Game/AjoutsQuentin/ThirdPersonQuentin` OtherActor))
  (set `/Game/AjoutsQuentin/ThirdPersonQuentin.CanTakeNote` false _asthird_person_quentin))

(event `ReadNote`
  (bind _returnvalue (`|CreateWidget` "/Game/AjoutsQuentin/Loot/Note.Note_C"))
  (`UserWidget.AddToViewport` _returnvalue 0)
  (`Image.SetBrush` (`/Game/AjoutsQuentin/Loot/Note.Image_49` _returnvalue) (make `SlateBrush` (32.0 32.0) (struct) (struct :`SpecifiedColor` (struct :`R` 1.0 :`G` 1.0 :`B` 1.0 :`A` 1.0) :`ColorUseRule` "UseColor_Specified") (struct :`CornerRadii` (struct :`W` 1.0) :`Color` (struct :`SpecifiedColor` (struct) :`ColorUseRule` "UseColor_Specified") :`RoundingType` "HalfHeightRadius") (`self.Note`)))
  (`GameplayStatics.PlaySound2D` "/Game/AjoutsQuentin/SoundDesignQuentin/Note_opening.Note_opening" 1.0 1.0 0.0 null null))

(event `Stop reading`
  (`/Game/AjoutsQuentin/Loot/Note.ReadingStop` (stale `ReadNote` _returnvalue))
  (`Widget.RemoveFromParent` (stale `ReadNote` _returnvalue))
  (`GameplayStatics.PlaySound2D` "/Game/AjoutsQuentin/SoundDesignQuentin/Note_Closing.Note_Closing" 1.0 1.0 0.0 null null))

(fn `UserConstructionScript`)
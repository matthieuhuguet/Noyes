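; AI_Distance_BP is a ranged enemy that turns to face the third-person character on sight and shoots at it.
; Pawn sensing drives the attack, spawning Projectile_BP at a spawn component, with a boolean and Delay limiting the fire rate.
; BeginPlay caches three patrol points and picks one at random.
; The timeline meant to lerp the enemy between those points is never triggered, so it does not patrol.
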(event `self.ReceiveBeginPlay`
  ;[1 1 1] Set Patrol Points
  (set `self.PatrolPoints` (`|MakeArray` (`SceneComponent.K2_GetComponentLocation` (`self.MovePosition1`)) (`SceneComponent.K2_GetComponentLocation` (`self.MovePosition2`)) (`SceneComponent.K2_GetComponentLocation` (`self.MovePosition3`))))
  (`self.Get random location`))

(event `self.PawnSensing.OnSeePawn`
  (params (Pawn :type "Pawn Object Reference"))
  ;[1 1 1] Look n Shoot
  (bind _asbp_third_person_character (cast `/Game/ThirdPerson/Blueprints/BP_ThirdPersonCharacter` Pawn))
  (`|ExecutionSequence`
    (:`then_0`
      (`self.K2_SetActorRotation` (`KismetMathLibrary.FindLookAtRotation` (`self.K2_GetActorLocation`) (`self.K2_GetActorLocation` _asbp_third_person_character))))
    (:`then_1`
      (if (`self.SpawnProjectile`)
        (`|SpawnActorFromClass` "/Game/ThirdPerson/Blueprints/Projectile_BP.Projectile_BP_C" (`SceneComponent.K2_GetComponentToWorld` (`self.ProjectileSpawnLocation`)) "Undefined" "OverrideRootScale" null null)
        (set `self.SpawnProjectile` false)
        (`KismetSystemLibrary.Delay` 1.5)
        (set `self.SpawnProjectile` true)))))

(fn `Get random location`
  (set `self.Current patrol Points` (`KismetMathLibrary.RandomInteger` (`KismetArrayLibrary.Array_Length` (`self.PatrolPoints`)))))

(fn `UserConstructionScript`)
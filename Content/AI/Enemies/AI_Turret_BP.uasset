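; AI turret enemy Blueprint with a Pawn Sensing component, meant to face the player and shoot projectiles.
; The look-and-shoot logic rotates the actor toward a BP_ThirdPersonCharacter and spawns Projectile_BP at ProjectileSpawnLocation, gated by a boolean and delay as a cooldown.
; That logic is disconnected from the empty On See Pawn event, so it never runs as saved.
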(event `self.PawnSensing.OnSeePawn`
  (params (Pawn :type "Pawn Object Reference"))
  ;[1 1 1] Look n Shoot
)

(fn `UserConstructionScript`)
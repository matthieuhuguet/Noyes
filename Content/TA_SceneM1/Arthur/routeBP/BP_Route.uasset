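; BP_Route is a spline-driven route actor that builds its geometry in the construction script, with no active runtime logic.
; Three sequential passes each add a spline mesh component per segment between neighboring spline points, producing three overlapping layers along the same path.
; Each segment runs along the X forward axis, takes its local positions and tangents from the spline, and has collision disabled.
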(fn `UserConstructionScript`
  (`|ExecutionSequence`
    (:`then_0`
      (for _index (range (+ (- (`SplineComponent.GetNumberOfSplinePoints` (`self.Spline`)) 2) 1))
        (bind _returnvalue (`AddComponent|NODE_AddSplineMeshComponent-0`))
        (`SplineMeshComponent.SetForwardAxis` _returnvalue "X" true)
        (`PrimitiveComponent.SetCollisionEnabled` _returnvalue "NoCollision")
        (bind _returnvalue_2 (+ _index 1))
        (`SplineMeshComponent.SetStartAndEnd` _returnvalue (`SplineComponent.GetLocationAtSplinePoint` (`self.Spline`) _index "Local") (`SplineComponent.GetTangentAtSplinePoint` (`self.Spline`) _index "Local") (`SplineComponent.GetLocationAtSplinePoint` (`self.Spline`) _returnvalue_2 "Local") (`SplineComponent.GetTangentAtSplinePoint` (`self.Spline`) _returnvalue_2 "Local") true)))
    (:`then_1`
      (for _index_2 (range (+ (- (`SplineComponent.GetNumberOfSplinePoints` (`self.Spline`)) 2) 1))
        (bind _returnvalue_3 (`AddComponent|NODE_AddSplineMeshComponent-3`))
        (`SplineMeshComponent.SetForwardAxis` _returnvalue_3 "X" true)
        (`PrimitiveComponent.SetCollisionEnabled` _returnvalue_3 "NoCollision")
        (bind _returnvalue_4 (+ _index_2 1))
        (`SplineMeshComponent.SetStartAndEnd` _returnvalue_3 (`SplineComponent.GetLocationAtSplinePoint` (`self.Spline`) _index_2 "Local") (`SplineComponent.GetTangentAtSplinePoint` (`self.Spline`) _index_2 "Local") (`SplineComponent.GetLocationAtSplinePoint` (`self.Spline`) _returnvalue_4 "Local") (`SplineComponent.GetTangentAtSplinePoint` (`self.Spline`) _returnvalue_4 "Local") true)))
    (:`then_2`
      (for _index_3 (range (+ (- (`SplineComponent.GetNumberOfSplinePoints` (`self.Spline`)) 2) 1))
        (bind _returnvalue_5 (`AddComponent|NODE_AddSplineMeshComponent-4`))
        (`SplineMeshComponent.SetForwardAxis` _returnvalue_5 "X" true)
        (`PrimitiveComponent.SetCollisionEnabled` _returnvalue_5 "NoCollision")
        (bind _returnvalue_6 (+ _index_3 1))
        (`SplineMeshComponent.SetStartAndEnd` _returnvalue_5 (`SplineComponent.GetLocationAtSplinePoint` (`self.Spline`) _index_3 "Local") (`SplineComponent.GetTangentAtSplinePoint` (`self.Spline`) _index_3 "Local") (`SplineComponent.GetLocationAtSplinePoint` (`self.Spline`) _returnvalue_6 "Local") (`SplineComponent.GetTangentAtSplinePoint` (`self.Spline`) _returnvalue_6 "Local") true)))))
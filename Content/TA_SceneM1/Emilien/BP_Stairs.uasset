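; BP_Stairs is a Geometry Script generated mesh Blueprint that procedurally builds a staircase.
; On each mesh rebuild, it appends one subdivided box per step along X, with height scaled by the step index to form solid rising steps.
; Box-projection UVs use configurable offset and scale, reapplied to the mesh after each append, and a leftover debug string prints when the loop ends.
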(event `self.OnRebuildGeneratedMesh`
  (params (TargetMesh :type "DynamicMesh Object Reference"))
  (bind (_stairsize_x _stairsize_y _stairsize_z) (`KismetMathLibrary.BreakVector` (`self.StairSize`)))
  (for _index (range 1 (+ (`self.Stairs Number`) 1))
    (bind _returnvalue (`GeometryScriptLibrary_MeshPrimitiveFunctions.AppendBox` TargetMesh (struct) (`KismetMathLibrary.MakeTransform` (`KismetMathLibrary.MakeVector` (* _stairsize_x _index)) (struct)) _stairsize_x _stairsize_y (* _stairsize_z _index) 10 10 10 "Base" null))
    (`GeometryScriptLibrary_MeshUVFunctions.SetMeshUVsFromBoxProjection` _returnvalue 0 (`KismetMathLibrary.MakeTransform` (`self.UV Offset`) (struct) (`self.UV Scale`)) 2 null))
  (`KismetSystemLibrary.PrintString` "Hello"))

(fn `UserConstructionScript`)
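; BP_House is a building Blueprint with optional balconies and shutters.
; Its construction script reads the Balcons and Volets booleans to show or hide four balcony components and one shutter component, without propagating to their children.
; The event graph holds only disabled placeholder events, so it adds no runtime logic.
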(fn `UserConstructionScript`
  (bind _balcon (`self.Balcon`))
  (bind _volets (`self.Volets`))
  (`|ExecutionSequence`
    (:`then_0`
      (if (`self.Balcons?`)
        (`SceneComponent.SetVisibility` _balcon true false)
        (`SceneComponent.SetVisibility` (`self.Balcon1`) true false)
        (`SceneComponent.SetVisibility` (`self.Balcon2`) true false)
        (`SceneComponent.SetVisibility` (`self.Balcon3`) true false)
        (else
          (`SceneComponent.SetVisibility` _balcon false false)
          (`SceneComponent.SetVisibility` (`self.Balcon1`) false false)
          (`SceneComponent.SetVisibility` (`self.Balcon2`) false false)
          (`SceneComponent.SetVisibility` (`self.Balcon3`) false false))))
    (:`then_1`
      (if (`self.Volets?`)
        (`SceneComponent.SetVisibility` _volets true false)
        (else
          (`SceneComponent.SetVisibility` _volets false false))))))
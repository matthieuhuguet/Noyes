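; PhareZone_BP is a spotlight detection zone that raises the third-person character's DetectionMeter while the player is detected.
; Tick-driven delays cycle the light and IsActive flag, roughly fifteen seconds on and five off.
; Player overlap sets detection only if active on entry, and any end overlap clears it, not the light switching off.
; While detected, a short delay throttles meter increments, shown through debug prints; the meter decrease logic is unconnected.
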(event `self.ReceiveTick`
  (params (DeltaSeconds :type "Float (single-precision)"))
  (`|ExecutionSequence`
    (:`then_0`
      (`KismetSystemLibrary.Delay` 15.0)
      (`SceneComponent.SetVisibility` (`self.SpotLight`) false false)
      (set `self.IsActive` false)
      (`KismetSystemLibrary.Delay` 5.0)
      (`SceneComponent.SetVisibility` (`self.SpotLight`) true false)
      (set `self.IsActive` true))
    (:`then_1`
      (if (`self.Player Detected`)
        (bind _asbp_third_person_character_final (cast `/Game/ThirdPerson/Blueprints/BP_ThirdPersonCharacter_Final` (`GameplayStatics.GetPlayerCharacter` 0)))
        (`KismetSystemLibrary.Delay` 0.1)
        (bind _output_get (set `/Game/ThirdPerson/Blueprints/BP_ThirdPersonCharacter_Final.Detection Meter` (+ (`/Game/ThirdPerson/Blueprints/BP_ThirdPersonCharacter_Final.Detection Meter` _asbp_third_person_character_final) 1) _asbp_third_person_character_final))
        (`KismetSystemLibrary.PrintString` (`KismetStringLibrary.Conv_IntToString` _output_get) true true (struct :`R` 0.575 :`A` 1.0) 1.0)))))

(event `self.ReceiveActorBeginOverlap`
  (params (OtherActor :type "Actor Object Reference"))
  (if (== OtherActor (`GameplayStatics.GetPlayerCharacter` 0))
    (if (`self.IsActive`)
      (set `self.Player Detected` true)
      (`KismetSystemLibrary.PrintString` "Gotcha"))))

(event `self.ReceiveActorEndOverlap`
  (params (OtherActor :type "Actor Object Reference"))
  (set `self.Player Detected` false)
  (`KismetSystemLibrary.PrintString` "Out of sight"))

(fn `UserConstructionScript`)
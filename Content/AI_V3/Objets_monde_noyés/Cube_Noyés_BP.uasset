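; Cube actor that exists only in the drowned world (Monde Noyés), one of that world's objects.
; It starts hidden on BeginPlay, then checks the MondeNoyés flag every Tick.
; Appear shows the actor and enables query and physics collision on the cube, while Dissapear hides it and turns collision off.
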(event `self.ReceiveBeginPlay`
  (`self.Dissapear`))

(event `Appear`
  (`self.SetActorHiddenInGame` false)
  (`PrimitiveComponent.SetCollisionEnabled` (`self.Cube`) "QueryAndPhysics"))

(event `Dissapear`
  (`self.SetActorHiddenInGame` true)
  (`PrimitiveComponent.SetCollisionEnabled` (`self.Cube`) "NoCollision"))

(event `self.ReceiveTick`
  (params (DeltaSeconds :type "Float (single-precision)"))
  (if (`self.Monde Noyés?`)
    (`self.Appear`)
    (else
      (`self.Dissapear`))))

(fn `UserConstructionScript`
  (`parent.UserConstructionScript`))
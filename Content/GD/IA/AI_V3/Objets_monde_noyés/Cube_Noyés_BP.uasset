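; Cube obstacle that is solid and visible only while the MondeNoyés (drowned world) flag is on, and starts hidden.
; Tick polls that flag every frame, toggling the cube's visibility and collision and hiding the translucent Translu component whenever the cube appears.
; Box overlaps with the deprecated third-person character show or hide Translu.
; Particle and glow-sound logic is left unconnected.
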(event `self.ReceiveBeginPlay`
  (`self.Dissapear`))

(event `Appear`
  (`SceneComponent.SetVisibility` (`self.Cube`) true false)
  (`PrimitiveComponent.SetCollisionEnabled` (`self.Cube`) "QueryAndPhysics")
  (`SceneComponent.SetVisibility` (`self.Translu`) false false))

(event `Dissapear`
  (`SceneComponent.SetVisibility` (`self.Cube`) false false)
  (`PrimitiveComponent.SetCollisionEnabled` (`self.Cube`) "NoCollision"))

(event `self.ReceiveTick`
  (params (DeltaSeconds :type "Float (single-precision)"))
  (if (`self.Monde Noyés?`)
    (`self.Appear`)
    (else
      (`self.Dissapear`))))

(event `self.Box.OnComponentBeginOverlap`
  (params (OverlappedComponent :type "PrimitiveComponent Object Reference") (OtherActor :type "Actor Object Reference") (OtherComp :type "PrimitiveComponent Object Reference") (OtherBodyIndex :type Integer) (bFromSweep :type Boolean) (SweepResult :type "HitResult Structure (by ref)"))
  (cast `/Game/GD/Blueprints/ThirdPerson/Blueprints/old/Deprecated_BP_ThirdPersonCharacter_Final` OtherActor)
  (`SceneComponent.SetVisibility` (`self.Translu`) true false))

(event `self.Box.OnComponentEndOverlap`
  (params (OverlappedComponent :type "PrimitiveComponent Object Reference") (OtherActor :type "Actor Object Reference") (OtherComp :type "PrimitiveComponent Object Reference") (OtherBodyIndex :type Integer))
  (cast `/Game/GD/Blueprints/ThirdPerson/Blueprints/old/Deprecated_BP_ThirdPersonCharacter_Final` OtherActor)
  (`SceneComponent.SetVisibility` (`self.Translu`) false false))

(fn `UserConstructionScript`
  (`parent.UserConstructionScript`))
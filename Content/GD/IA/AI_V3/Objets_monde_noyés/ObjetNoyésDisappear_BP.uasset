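; Object for the "Monde Noyés" (drowned world) mechanic that disappears while the drowned-world flag is active and is present otherwise.
; It starts visible, then checks the MondeNoyés boolean every Tick to call its Appear or Dissapear event.
; These events toggle the static mesh's visibility and collision together, without propagating visibility to child components.
; Nothing in this graph sets the flag.
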(event `self.ReceiveBeginPlay`
  (`self.Appear`))

(event `Appear`
  (bind _staticmesh (`self.StaticMesh`))
  (`SceneComponent.SetVisibility` _staticmesh true false)
  (`PrimitiveComponent.SetCollisionEnabled` _staticmesh "QueryAndPhysics"))

(event `Dissapear`
  (bind _staticmesh (`self.StaticMesh`))
  (`SceneComponent.SetVisibility` _staticmesh false false)
  (`PrimitiveComponent.SetCollisionEnabled` _staticmesh "NoCollision"))

(event `self.ReceiveTick`
  (params (DeltaSeconds :type "Float (single-precision)"))
  (if (`self.Monde Noyés?`)
    (`self.Dissapear`)
    (else
      (`self.Appear`))))

(fn `UserConstructionScript`
  (`parent.UserConstructionScript`))
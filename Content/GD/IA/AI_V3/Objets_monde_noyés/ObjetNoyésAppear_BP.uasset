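; Blueprint for a drowned-world ("Noyés") object that appears at BeginPlay with an opacity fade.
; It applies a dynamic M_Noye material to three mesh slots, enables visibility and collision, and drives Opacity through a timeline.
; A five-second Delay on the timeline's Update reverses the fade without disabling collision.
; Dissapear hides the mesh and disables collision, but its only caller, a MondeNoyés check, never runs.
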(event `self.ReceiveBeginPlay`
  (bind _returnvalue (`KismetMaterialLibrary.CreateDynamicMaterialInstance` "/Game/GD/IA/AI_V3/Objets_monde_noyés/M_Noye.M_Noye"))
  (set `self.NoyéMaterial` _returnvalue)
  (`self.Opacity`)
  (`self.Appear`))

(event `Appear`
  (bind _staticmesh (`self.StaticMesh`))
  (`SceneComponent.SetVisibility` _staticmesh true false)
  (`PrimitiveComponent.SetCollisionEnabled` _staticmesh "QueryAndPhysics"))

(event `Opacity`
  (bind _staticmesh (`self.StaticMesh`))
  (bind `_noyématerial` (`self.NoyéMaterial`))
  ;[1 1 1] Change Opacity
  (`PrimitiveComponent.SetMaterial` _staticmesh 0 `_noyématerial`)
  (`PrimitiveComponent.SetMaterial` _staticmesh 1 `_noyématerial`)
  (`PrimitiveComponent.SetMaterial` _staticmesh 2 `_noyématerial`)
  (`self.Appear`)
  (bind (_direction _newtrack_0) (`Timeline|Timeline_0` :!label _label)
    (:`Update`
      (`MaterialInstanceDynamic.SetScalarParameterValue` (`self.NoyéMaterial`) "Opacity" _newtrack_0)
      (`KismetSystemLibrary.Delay` 5.0)
      (goto _label :!via `Reverse`))))

(event `Dissapear`
  (bind _staticmesh (`self.StaticMesh`))
  (`SceneComponent.SetVisibility` _staticmesh false false)
  (`PrimitiveComponent.SetCollisionEnabled` _staticmesh "NoCollision"))

(fn `UserConstructionScript`
  (`parent.UserConstructionScript`))
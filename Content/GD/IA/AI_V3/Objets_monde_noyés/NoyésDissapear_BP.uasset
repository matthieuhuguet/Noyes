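; Actor Blueprint for an object that disappears while the MondeNoyés (drowned world) flag is true and is present otherwise.
; BeginPlay calls Appear, then Tick re-reads the flag every frame and calls Disappear or Appear without checking for a change.
; These two events toggle the actor's hidden state and switch the StaticMesh collision between query-and-physics and none.
; Nothing in these graphs sets the flag.
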(event `self.ReceiveBeginPlay`
  (`self.Appear`))

(event `Appear`
  (`self.SetActorHiddenInGame` false)
  (`PrimitiveComponent.SetCollisionEnabled` (`self.StaticMesh`) "QueryAndPhysics"))

(event `Disappear`
  (`self.SetActorHiddenInGame` true)
  (`PrimitiveComponent.SetCollisionEnabled` (`self.StaticMesh`) "NoCollision"))

(event `self.ReceiveTick`
  (params (DeltaSeconds :type "Float (single-precision)"))
  (if (`self.Monde Noyés?`)
    (`self.Disappear`)
    (else
      (`self.Appear`))))

(fn `UserConstructionScript`
  (`parent.UserConstructionScript`))
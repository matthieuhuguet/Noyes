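; Blueprint for a world object that exists only in the "Monde Noyés" (drowned world) state, appearing and disappearing with it.
; It starts hidden on BeginPlay, then checks the MondeNoyés boolean every Tick to call the Appear or Dissapear event.
; These events toggle the static mesh's visibility and switch its collision between query-and-physics and none.
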(event `self.ReceiveBeginPlay`
  (`self.Dissapear`))

(event `Appear`
  (bind _staticmesh (`self.StaticMesh`))
  (`SceneComponent.SetVisibility` _staticmesh true false)
  (`PrimitiveComponent.SetCollisionEnabled` _staticmesh "QueryAndPhysics"))

(event `Dissapear`
  (bind _staticmesh (`self.StaticMesh`))
  (`SceneComponent.SetVisibility` _staticmesh false false)
  (`PrimitiveComponent.SetCollisionEnabled` _staticmesh "NoCollision"))

(event `self.ReceiveTick`
  (params (DeltaSeconds :type "Float (single-precision)"))
  (if (`self.Monde Noyés?`)
    (`self.Appear`)
    (else
      (`self.Dissapear`))))

(fn `UserConstructionScript`
  (`parent.UserConstructionScript`))
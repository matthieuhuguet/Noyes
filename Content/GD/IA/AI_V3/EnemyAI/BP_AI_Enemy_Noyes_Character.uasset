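; Enemy AI character with a random mask that detects the player, takes damage and drops ammo on death.
; Pawn sensing and proximity spheres drive a timeline detection meter, alerting music and blackboard when full.
; Each state update rewrites all blackboard flags, leaving only the passed state true for the behavior tree.
; Damage updates life widget and hit marker, applies knockback and montage; death stops AI, fades meshes and destroys the actor.
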(event `self.ReceiveBeginPlay`
  ;[0.3278 0.9216 1] Define Player And Start Playing
  (`SkeletalMeshComponent.LinkAnimClassLayers` (`self.Mesh`) "/Game/GD/CharactersEffects/Heroes/Mannequin/Animations/Locomotion/Unarmed/ABP_UnarmedAnimLayers.ABP_UnarmedAnimLayers_C")
  (bind _noyescharacter (`/Game/GD/Blueprints_Function_Library/BFL_Player.Get Player Character`))
  (`self.SetValueAsObject` _noyescharacter "Player")
  (`KismetSystemLibrary.Delay` 0.2)
  (`self.SetStateBooleanOfBlackboard` true)
  (bind _noyescharacter_2 (`/Game/GD/Blueprints_Function_Library/BFL_Player.Get Player Character`))
  (set `self.Noyes Character` _noyescharacter_2)
  (bind _aslife_ennemy (cast `/Game/GD/UI_HUD/Life_Ennemy` (`WidgetComponent.GetUserWidgetObject` (`self.Widget_Life`))))
  (set `/Game/GD/UI_HUD/Life_Ennemy.CurrentLifeUI` (`self.Current Health`) _aslife_ennemy)
  (set `/Game/GD/UI_HUD/Life_Ennemy.MaxLifeUI` (`self.Current Health`) _aslife_ennemy))

(event `self.ReceiveTick`
  (params (DeltaSeconds :type "Float (single-precision)")))

(event `AttackAI`
  (bind _returnvalue (`self.K2_GetActorLocation`))
  ;[0.3278 0.9216 1] Attack AI
  (bind _outhit (`KismetSystemLibrary.SphereTraceSingleByProfile` :`Start` _returnvalue :`End` (+ _returnvalue (* (`self.GetActorForwardVector`) 75.0)) :`Radius` 15.0 :`DrawDebugType` "ForDuration" :`DrawTime` 2.0))
  (bind (_bblockinghit _binitialoverlap _time _distance _location _impactpoint _normal _impactnormal _physmat _hitactor) (`GameplayStatics.BreakHitResult` _outhit))
  (if _bblockinghit
    (bind _asbp_noyes_character (cast `/Game/GD/BP_Controller_GameMode_MainCharacter_GameInstance/BP_Noyes_Character` _hitactor))))

(event `HearNoiseTrigger`
  ;[0.5089 0.4452 1] The noise make the AI to Search Phase
  (cast `/Game/GD/BP_Controller_GameMode_MainCharacter_GameInstance/BP_Noyes_Character` (stale `self.PawnSensing.OnHearNoise` Instigator) :!label _label)
  (`self.AddDetection`)
  (`self.SetStateBooleanOfBlackboard` false false false false false true)
  (`self.CheckConditionPlayerIsDetected`))

(event `self.PawnSensing.OnHearNoise`
  (params (Instigator :type "Pawn Object Reference") (Location :type "Vector Structure (by ref)") (Volume :type "Float (single-precision)"))
  ;[0.5089 0.4452 1] The noise make the AI to Search Phase
  (`self.LastKnownLocation`)
  (`KismetSystemLibrary.PrintString` "hear")
  (if (not (`/Game/GD/BP_Controller_GameMode_MainCharacter_GameInstance/BP_Noyes_Character.IsCrouch` (`self.Noyes Character`)))
    (goto _label)))

(event `self.PawnSensing.OnSeePawn`
  (params (Pawn :type "Pawn Object Reference"))
  ;[0.5089 0.4452 1] See Pawn
  (set `self.Sight` true)
  (`self.LastKnownLocation`)
  (`KismetSystemLibrary.PrintString` "See")
  (cast `/Game/GD/BP_Controller_GameMode_MainCharacter_GameInstance/BP_Noyes_Character` Pawn)
  (`self.AddDetection`)
  (`self.SetStateBooleanOfBlackboard` false false false false false true)
  (`self.CheckConditionPlayerIsDetected`))

(event `UpdateLife&UI`
  (params (InputPin :type "Float (double-precision)"))
  (bind _returnvalue (`KismetMathLibrary.Conv_IntToDouble` (`KismetMathLibrary.Conv_Int64ToInt` (`KismetMathLibrary.Conv_DoubleToInt64` (- (`self.Current Health`) InputPin)))))
  ;[1 1 1] UI
  (bind _aslife_ennemy (cast `/Game/GD/UI_HUD/Life_Ennemy` (`WidgetComponent.GetUserWidgetObject` (`self.Widget_Life`))))
  (`/Engine/EditorBlueprintResources/StandardMacros.IsValid` _aslife_ennemy
    (:`Is Valid`
      (set `/Game/GD/UI_HUD/Life_Ennemy.CurrentLifeUI` _returnvalue _aslife_ennemy)
      (set `self.Current Health` _returnvalue))))

(event `self.ReceiveAnyDamage`
  (params (Damage :type "Float (single-precision)") (DamageType :type "DamageType Object Reference") (InstigatedBy :type "Controller Object Reference") (DamageCauser :type "Actor Object Reference"))
  (bind _anim_montage_ennemy (`self.Anim Montage Ennemy`))
  ;[0.5089 0.4452 1] Event Any Damage
  (`self.LastKnownLocation`)
  (`self.UpdateLife&UI` Damage)
  (`|ExecutionSequence`
    (:`then_0`
      (bind _noyescharacter (`/Game/GD/Blueprints_Function_Library/BFL_Player.Get Player Character`))
      ;[0.5089 0.4452 1] Push Character When Receive Damage
      (`self.SetStateBooleanOfBlackboard` false false false true)
      (`self.LaunchCharacter` (* (`KismetMathLibrary.GetForwardVector` (`self.K2_GetActorRotation` _noyescharacter)) 500.0))
      (`self.PlayAnimMontage` (`|GetArrayItem` _anim_montage_ennemy (`KismetMathLibrary.RandomIntegerInRange` 0 (- (`KismetArrayLibrary.Array_Length` _anim_montage_ennemy) 1))))
      (`self.SelectorOfHitMarker`))
    (:`then_1`
      ;[1 1 1] Death Kill actor
      (if (<= (`self.Current Health`) 0.0)
        (`CharacterMovementComponent.DisableMovement` (`self.CharacterMovement`))
        (`self.PlayDeathSound`)
        (`self.Drop Munition`)
        (`SkeletalMeshComponent.OverrideAnimationData` (`self.Mesh`) "/Game/GD/Enemy/Enemy_Anims/ReactAnims/AM_EnemyDeath.AM_EnemyDeath" false true 0.0 1.0)
        (`self.StopLogic`) ; Hope this work test for bug
        (`self.SetOffWidgets`)
        (`KismetSystemLibrary.Delay` 1.0)
        (bind (_direction _newtrack_0) (`Timeline|Timeline_2`)
          (:`Update`
            (`MeshComponent.SetScalarParameterValueOnMaterials` (`self.Mesh`) "Opacity" (`KismetMathLibrary.Lerp` 1.0 0.0 _newtrack_0))
            (`MeshComponent.SetScalarParameterValueOnMaterials` (`self.MasqueMesh`) "Opacity" (`KismetMathLibrary.Lerp` 1.0 0.0 _newtrack_0)))
          (:`Finished`
            (`self.K2_DestroyActor`)))))))

(event `SelectorOfHitMarker`
  (bind _returnvalue (<= (`self.Current Health`) 0.0))
  (`KismetSystemLibrary.DelayUntilNextTick`)
  (bind _asbp_hud_noyes (`/Game/GD/Blueprints_Function_Library/BFL_HUD.Get_HUD_Noyes`))
  (bind _asumg_all (cast `/Game/GD/UI_HUD/UMG_All` (`/Game/GD/BP_Controller_GameMode_MainCharacter_GameInstance/BP_HUD_Noyes.WBP_UMG_All_Object` _asbp_hud_noyes)))
  (if _returnvalue
    (bind _crosshair (`/Game/GD/UI_HUD/UMG_All.CrossHair` _asumg_all))
    (`/Game/GD/UI_HUD/UserCreatedUMGForCustom/CrossHair.HitMarker` _crosshair _returnvalue)
    (else
      (`/Game/GD/UI_HUD/UserCreatedUMGForCustom/CrossHair.HitMarker` _crosshair false))))

(event `StopLogic`
  ;[1 1 1] Death Kill actor
  (`BrainComponent.StopLogic` (`AIController.BrainComponent` (`AIBlueprintHelperLibrary.GetAIController` self)) "IsDead"))

(event `/Game/GD/Blueprints/ThirdPerson/Blueprints/BPI_Character.Interact`
  ;[1 1 1] Interact Is Punch
  (`self.HitPunchMarker`))

(event `HitPunchMarker`
  (bind _returnvalue (<= (`self.Current Health`) 0.0))
  ;[1 1 1] Punched Play Animation
  (`KismetSystemLibrary.DelayUntilNextTick`) ; Compute Damage
  (bind _ashit_marker_punch (cast `/Game/GD/UI_HUD/UserCreatedUMGForCustom/HitMarkerPunch` (`WidgetComponent.GetWidget` (`self.Widget_Hit`))))
  (if _returnvalue
    (`/Game/GD/UI_HUD/UserCreatedUMGForCustom/HitMarkerPunch.HitMarker` _ashit_marker_punch _returnvalue)
    (else
      (`/Game/GD/UI_HUD/UserCreatedUMGForCustom/HitMarkerPunch.HitMarker` _ashit_marker_punch false))))

(event `self.SphereCollisionPlayerRange.OnComponentBeginOverlap`
  (params (OverlappedComponent :type "PrimitiveComponent Object Reference") (OtherActor :type "Actor Object Reference") (OtherComp :type "PrimitiveComponent Object Reference") (OtherBodyIndex :type Integer) (bFromSweep :type Boolean) (SweepResult :type "HitResult Structure (by ref)"))
  ;[0.9823 1 0.4678] On enter define player | On exit Player = Blank | Comment faire pour que le joueur ne tue pas les ennemis de trop loin ?
  (cast `/Game/GD/BP_Controller_GameMode_MainCharacter_GameInstance/BP_Noyes_Character` OtherActor)
  (`self.Set Value As Bool` "IsPlayerInRange?" true)
  (set `self.PlayerInRangeLocal` true))

(event `self.SphereCollisionPlayerRange.OnComponentEndOverlap`
  (params (OverlappedComponent :type "PrimitiveComponent Object Reference") (OtherActor :type "Actor Object Reference") (OtherComp :type "PrimitiveComponent Object Reference") (OtherBodyIndex :type Integer))
  ;[0.9823 1 0.4678] On enter define player | On exit Player = Blank | Comment faire pour que le joueur ne tue pas les ennemis de trop loin ?
  (cast `/Game/GD/BP_Controller_GameMode_MainCharacter_GameInstance/BP_Noyes_Character` OtherActor)
  (`self.Set Value As Bool` "IsPlayerInRange?")
  (set `self.PlayerInRangeLocal` false)
  (`self.SetStateBooleanOfBlackboard` false false false false true)
  (`self.RemoveDetection`)
  (set `self.Sight` false))

(event `Drop Munition`
  (`|SpawnActorFromClass` "/Game/Environment_TA/Assets/Props/Munitions/BP_Boite_munition.BP_Boite_munition_C" (`KismetMathLibrary.MakeTransform` (- (`self.K2_GetActorLocation`) (0.0 0.0 90.0)) (`self.K2_GetActorRotation`)) "Undefined" "OverrideRootScale" null null))

(event `self.SphereCollisionDetectPlayer.OnComponentBeginOverlap`
  (params (OverlappedComponent :type "PrimitiveComponent Object Reference") (OtherActor :type "Actor Object Reference") (OtherComp :type "PrimitiveComponent Object Reference") (OtherBodyIndex :type Integer) (bFromSweep :type Boolean) (SweepResult :type "HitResult Structure (by ref)"))
  ;[0.9823 1 0.4678] Medium Range
  (cast `/Game/GD/BP_Controller_GameMode_MainCharacter_GameInstance/BP_Noyes_Character` OtherActor)
  (if (`self.Sight`)
    (`TimelineComponent.SetPlaybackPosition` (`self.Timeline_0`) 3.0 true true)
    (`self.HearNoiseTrigger`)))

(event `self.SphereCriticalCrouchDetect.OnComponentBeginOverlap`
  (params (OverlappedComponent :type "PrimitiveComponent Object Reference") (OtherActor :type "Actor Object Reference") (OtherComp :type "PrimitiveComponent Object Reference") (OtherBodyIndex :type Integer) (bFromSweep :type Boolean) (SweepResult :type "HitResult Structure (by ref)"))
  ;[0.9823 1 0.4678] On Critical Range Call Hear Trigger and alert ennemy
  (cast `/Game/GD/BP_Controller_GameMode_MainCharacter_GameInstance/BP_Noyes_Character` OtherActor)
  (`self.HearNoiseTrigger`)
  (`TimelineComponent.SetPlaybackPosition` (`self.Timeline_0`) 3.0 true true))

(event `LastKnownLocation`
  ;[1 0.5647 1] Last Known Position
  (bind _noyescharacter (`/Game/GD/Blueprints_Function_Library/BFL_Player.Get Player Character`))
  (set `self.LastKnownPosition` (`self.K2_GetActorLocation` _noyescharacter)))

(event `Display ? Icon`
  (bind _widget_losesight (`self.Widget_LoseSight`))
  ;[1 0.5647 1] Display ? Icon for a while
  (`SceneComponent.SetVisibility` _widget_losesight true false)
  (`KismetSystemLibrary.Delay` 1.0)
  (`SceneComponent.SetVisibility` _widget_losesight false false))

(event `TimelineRotation`
  ;[0.5906 1 0.521] Behavior Tree
  (bind (_direction _alpha1) (`Timeline|Timeline_1` :!via `PlayFromStart`)
    (:`Update`
      (set `self.Alpha 2Rotation` _alpha1))))

(event `AddDetection`
  ;[0.5906 1 0.521] Behavior Tree
  (bind (_direction _alpha1) (`Timeline|Timeline_0` :!label _label_2)
    (:`Update`
      (set `self.Alpha 1` _alpha1)
      (`self.SetDetectionCurve` (`self.Alpha 1`)))))

(event `RemoveDetection`
  ;[0.5906 1 0.521] Behavior Tree
  (goto _label_2 :!via `Reverse`))

(event `CheckConditionPlayerIsDetected`
  ;[0.5906 1 0.521] Behavior Tree
  (`self.ResetDetection`)
  (if (== (`self.Alpha 1`) 1.0)
    (`self.Detected!`)
    (`self.SetStateBooleanOfBlackboard` false true)
    (message `/Game/GD/Audio/MusiquePhebusMogulusDarius/BPI_Music.Change Music State` (`GameplayStatics.GetGameState`) 2.0)))

(event `Detected!`
  ;[0.5906 1 0.521] Behavior Tree
  (`/Engine/EditorBlueprintResources/StandardMacros.DoOnce` false :!label _label_3 ; Reset later
    (:`Completed`
      (`/Game/GD/Blueprints_Function_Library/BFL_GameInstance.Get_GameInstance`))))

(event `ResetDetection`
  ;[0.5906 1 0.521] Behavior Tree
  (if (< (`self.Alpha 1`) 1.0)
    (goto _label_3 :!via `Reset`)))

(fn `DamagedActualActor`
  (returns (ActorDamaged :type "Actor Object Reference"))
  (return null))

(fn `GetAlphaOnOffForArm`
  (returns (AlphaParameter :type Boolean))
  (return false))

(fn `GetIsPlayingCombo`
  (returns (`Combo?` :type Boolean))
  (return false))

(fn `GetWeaponSocket`
  (params (SocketName :type Name))
  (returns (SocketTransform :type "Transform Structure"))
  (return))

(fn `PlayDeathSound`
  (`GameplayStatics.PlaySoundAtLocation` "/Game/GD/Audio/SFX/DeathMan/SC_DeathMan.SC_DeathMan" (`self.K2_GetActorLocation`) (struct) 1.0 1.0 0.0 "/Game/GD/Audio/SFX/SA_Main.SA_Main" null null null))

(fn `Set Value As Bool`
  (params (`Make Literal Name` :type "Name (by ref)") (BoolValue :type Boolean))
  (bind _returnvalue (`AIBlueprintHelperLibrary.GetBlackboard` (`AIBlueprintHelperLibrary.GetAIController` self)))
  (`/Engine/EditorBlueprintResources/StandardMacros.IsValid` _returnvalue
    (:`Is Valid`
      (`BlackboardComponent.SetValueAsBool` _returnvalue `Make Literal Name` BoolValue)
      (message `/Game/GD/Audio/MusiquePhebusMogulusDarius/BPI_Music.Change Music State` (`GameplayStatics.GetGameState`) 1.0))))

(fn `SetDetectionCurve`
  (params (Alpha :type "Float (double-precision)"))
  (bind _aswb_detection_enemy (cast `/Game/GD/UI_HUD/WB_Detection_Enemy` (`WidgetComponent.GetUserWidgetObject` (`self.Widget_Detection`))))
  (set `/Game/GD/UI_HUD/WB_Detection_Enemy.CurrentPercentDetection` (`KismetMathLibrary.Lerp` 0.0 1.0 Alpha) _aswb_detection_enemy))

(fn `SetOffWidgets`
  (`SceneComponent.SetVisibility` (`self.Widget_Alerted`) false false)
  (`SceneComponent.SetVisibility` (`self.Widget_Life`) false false)
  (`SceneComponent.SetVisibility` (`self.Widget_Detection`) false false)
  (`SceneComponent.SetVisibility` (`self.Widget_LoseSight`) false false))

(fn `SetStateBooleanOfBlackboard`
  (params (RoamingState :type Boolean) (`hasSeenPlayer?` :type Boolean) (`hasHearPlayer?` :type Boolean) (`hasReceiveDamage?` :type Boolean) (`LoseSightState?` :type Boolean) (`IsSuspicious?` :type Boolean))
  (bind _returnvalue (`AIBlueprintHelperLibrary.GetBlackboard` (`AIBlueprintHelperLibrary.GetAIController` self)))
  (`/Engine/EditorBlueprintResources/StandardMacros.IsValid` _returnvalue
    (:`Is Valid`
      (`BlackboardComponent.SetValueAsBool` _returnvalue "RoamingState" RoamingState)
      (`BlackboardComponent.SetValueAsBool` _returnvalue "hasSeenPlayer?" `hasSeenPlayer?`)
      (`BlackboardComponent.SetValueAsBool` _returnvalue "hasHearPlayer?" `hasHearPlayer?`)
      (`BlackboardComponent.SetValueAsBool` _returnvalue "hasReceiveDamage?" `hasReceiveDamage?`)
      (`BlackboardComponent.SetValueAsBool` _returnvalue "LoseSightState?" `LoseSightState?`)
      (`BlackboardComponent.SetValueAsBool` _returnvalue "IsSuspicious?" `IsSuspicious?`)
      (return))))

(fn `SetValueAsObject`
  (params (ObjectValue :type "Object Object Reference") (`Make Literal Name` :type "Name (by ref)"))
  (`BlackboardComponent.SetValueAsObject` (`AIBlueprintHelperLibrary.GetBlackboard` (`AIBlueprintHelperLibrary.GetAIController` self)) `Make Literal Name` ObjectValue))

(fn `UpdateLifeEnnemy`
  (returns (Guard_EnemyLife :type "Float (double-precision)"))
  (return 0.0))

(fn `UpdateLifeWidget`
  (params (DamageRecipient :type "Float (double-precision)"))
  (bind _current_health (`self.Current Health`))
  (bind _returnvalue (`KismetMathLibrary.Lerp` _current_health (- _current_health DamageRecipient)))
  (bind _aslife_ennemy (cast `/Game/GD/UI_HUD/Life_Ennemy` (`WidgetComponent.GetUserWidgetObject` (`self.Widget_Life`))))
  (`/Engine/EditorBlueprintResources/StandardMacros.IsValid` _aslife_ennemy
    (:`Is Valid`
      (set `/Game/GD/UI_HUD/Life_Ennemy.CurrentLifeUI` _returnvalue _aslife_ennemy)
      (set `self.Current Health` _returnvalue))))

(fn `UserConstructionScript`
  (`SkinnedMeshComponent.SetSkinnedAssetAndUpdate` (`self.Mesh`) "/Game/GD/Enemy/Lard/LardRig2.LardRig2" true)
  (`StaticMeshComponent.SetStaticMesh` (`self.MasqueMesh`) (select `int` (`KismetMathLibrary.RandomIntegerInRange` 0 2) :`0` "/Game/GD/Enemy/Masques/Scaphandre/_Scaphandre_UE5._Scaphandre_UE5" :`1` "/Game/GD/Enemy/Masques/Soudeur/_Soudeur_UE5._Soudeur_UE5" :`2` "/Game/GD/Enemy/Masques/Bioshock/Bioshock_.Bioshock_" :!type "StaticMesh Object Reference"))
  (set `self.Current Health` (`self.Current Health`)))
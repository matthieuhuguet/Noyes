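; Enemy AI character that turns sight, hearing, proximity and damage events into Blackboard keys, starting in a roaming state.
; Pawn sensing and damage call one setter that rewrites all five state flags; a sphere overlap flags player range and lost sight.
; While the player is in range, Tick records their last position.
; Damage updates the health widget, launches the enemy and plays a random montage; the detection-meter timeline is disconnected.
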(event `self.ReceiveTick`
  (params (DeltaSeconds :type "Float (single-precision)"))
  (if (`self.PlayerInRangeLocal`)
    (`self.LastKnownLocation`)))

(event `LoseDetection`)

(event `StartTimeline`)

(event `StopDetection`)

(event `self.ReceiveBeginPlay`
  ;[0.5906 1 0.521] Define Player And Start Playing
  (`SkeletalMeshComponent.LinkAnimClassLayers` (`self.Mesh`) "/Game/GD/CharactersEffects/Heroes/Mannequin/Animations/Locomotion/Unarmed/ABP_UnarmedAnimLayers.ABP_UnarmedAnimLayers_C")
  (bind _noyescharacter (`/Game/GD/Blueprints_Function_Library/BFL_Player.Get Player Character`))
  (`self.SetValueAsObject` _noyescharacter "Player")
  (`KismetSystemLibrary.Delay` 0.2)
  (`self.SetStateBooleanOfBlackboard` true))

(event `self.PawnSensing.OnHearNoise`
  (params (Instigator :type "Pawn Object Reference") (Location :type "Vector Structure (by ref)") (Volume :type "Float (single-precision)"))
  ;[0.5089 0.4452 1] The noise make the AI to Search Phase
  (cast `/Game/GD/BP_Controller_GameMode_MainCharacter_GameInstance/BP_Noyes_Character` Instigator)
  (`self.StartTimeline`)
  (`self.SetStateBooleanOfBlackboard` false false false false true))

(event `self.Sphere.OnComponentBeginOverlap`
  (params (OverlappedComponent :type "PrimitiveComponent Object Reference") (OtherActor :type "Actor Object Reference") (OtherComp :type "PrimitiveComponent Object Reference") (OtherBodyIndex :type Integer) (bFromSweep :type Boolean) (SweepResult :type "HitResult Structure (by ref)"))
  ;[0.3515 0.552 1] On enter define player | On exit Player = Blank | Comment faire pour que le joueur ne tue pas les ennemis de trop loin ?
  (cast `/Game/GD/BP_Controller_GameMode_MainCharacter_GameInstance/BP_Noyes_Character` OtherActor)
  (`self.Set Value As Bool` "IsPlayerInRange?" true)
  (set `self.PlayerInRangeLocal` true))

(event `self.PawnSensing.OnSeePawn`
  (params (Pawn :type "Pawn Object Reference"))
  ;[0.3278 0.9216 1] See Pawn
  (cast `/Game/GD/BP_Controller_GameMode_MainCharacter_GameInstance/BP_Noyes_Character` Pawn)
  (`self.StartTimeline`)
  (`self.SetStateBooleanOfBlackboard` false true))

(event `self.Sphere.OnComponentEndOverlap`
  (params (OverlappedComponent :type "PrimitiveComponent Object Reference") (OtherActor :type "Actor Object Reference") (OtherComp :type "PrimitiveComponent Object Reference") (OtherBodyIndex :type Integer))
  ;[0.3515 0.552 1] On enter define player | On exit Player = Blank | Comment faire pour que le joueur ne tue pas les ennemis de trop loin ?
  (cast `/Game/GD/BP_Controller_GameMode_MainCharacter_GameInstance/BP_Noyes_Character` OtherActor)
  (`self.Set Value As Bool` "IsPlayerInRange?")
  (set `self.PlayerInRangeLocal` false)
  (`self.Set Value As Bool` "LoseSightState?" true))

(event `self.ReceiveAnyDamage`
  (params (Damage :type "Float (single-precision)") (DamageType :type "DamageType Object Reference") (InstigatedBy :type "Controller Object Reference") (DamageCauser :type "Actor Object Reference"))
  (bind _anim_montage_ennemy (`self.Anim Montage Ennemy`))
  ;[1 0.4179 0.4179] Event Any Damage
  (`self.UpdateLifeWidget` Damage)
  (bind _noyescharacter (`/Game/GD/Blueprints_Function_Library/BFL_Player.Get Player Character`))
  (`|ExecutionSequence`
    (:`then_0`
      ;[0.5089 0.4452 1] Push Character When Receive Damage
      (`self.LaunchCharacter` (* (`KismetMathLibrary.GetForwardVector` (`self.K2_GetActorRotation` _noyescharacter)) 1500.0))
      (`self.PlayAnimMontage` (`|GetArrayItem` _anim_montage_ennemy (`KismetMathLibrary.RandomIntegerInRange` 0 (- (`KismetArrayLibrary.Array_Length` _anim_montage_ennemy) 1)))))
    (:`then_1`
      (`self.SetStateBooleanOfBlackboard` false false false true))))

(event `LastKnownLocation`
  ;[0.9823 1 0.4678] Last Known Position
  (bind _noyescharacter (`/Game/GD/Blueprints_Function_Library/BFL_Player.Get Player Character`))
  (set `self.LastKnownPosition` (`self.K2_GetActorLocation` _noyescharacter)))

(event `Display ? Icon`
  (bind _widget_losesight (`self.Widget_LoseSight`))
  ;[1 0.5647 1] Display ? Icon for a while
  (`SceneComponent.SetVisibility` _widget_losesight true false)
  (`KismetSystemLibrary.Delay` 1.0)
  (`SceneComponent.SetVisibility` _widget_losesight false false))

(fn `Set Value As Bool`
  (params (`Make Literal Name` :type "Name (by ref)") (BoolValue :type Boolean))
  (`BlackboardComponent.SetValueAsBool` (`AIBlueprintHelperLibrary.GetBlackboard` (`AIBlueprintHelperLibrary.GetAIController` self)) `Make Literal Name` BoolValue))

(fn `SetDetectionCurve`
  (params (Alpha :type "Float (double-precision)"))
  (bind _aswb_detection_enemy (cast `/Game/GD/UI_HUD/WB_Detection_Enemy` (`WidgetComponent.GetUserWidgetObject` (`self.Widget_Detection`))))
  (set `/Game/GD/UI_HUD/WB_Detection_Enemy.CurrentPercentDetection` (`KismetMathLibrary.Lerp` 0.0 1.0 Alpha) _aswb_detection_enemy))

(fn `SetStateBooleanOfBlackboard`
  (params (RoamingState :type Boolean) (`hasSeenPlayer?` :type Boolean) (`hasHearPlayer?` :type Boolean) (`hasReceiveDamage?` :type Boolean) (`isInvestigating?` :type Boolean))
  (bind _returnvalue (`AIBlueprintHelperLibrary.GetBlackboard` (`AIBlueprintHelperLibrary.GetAIController` self)))
  (`BlackboardComponent.SetValueAsBool` _returnvalue "RoamingState" RoamingState)
  (`BlackboardComponent.SetValueAsBool` _returnvalue "hasSeenPlayer?" `hasSeenPlayer?`)
  (`BlackboardComponent.SetValueAsBool` _returnvalue "hasHearPlayer?" `hasHearPlayer?`)
  (`BlackboardComponent.SetValueAsBool` _returnvalue "hasReceiveDamage?" `hasReceiveDamage?`)
  (`BlackboardComponent.SetValueAsBool` _returnvalue "isInvestigating?" `isInvestigating?`)
  (return))

(fn `SetValueAsObject`
  (params (ObjectValue :type "Object Object Reference") (`Make Literal Name` :type "Name (by ref)"))
  (`BlackboardComponent.SetValueAsObject` (`AIBlueprintHelperLibrary.GetBlackboard` (`AIBlueprintHelperLibrary.GetAIController` self)) `Make Literal Name` ObjectValue))

(fn `UpdateLifeWidget`
  (params (DamageRecipient :type "Float (double-precision)"))
  (bind _returnvalue (- (`self.Current Health`) DamageRecipient))
  (bind _aslife_ennemy (cast `/Game/GD/UI_HUD/Life_Ennemy` (`WidgetComponent.GetUserWidgetObject` (`self.Widget_Life`))))
  (`/Engine/EditorBlueprintResources/StandardMacros.IsValid` _aslife_ennemy
    (:`Is Valid`
      (set `/Game/GD/UI_HUD/Life_Ennemy.CurrentLifeUI` _returnvalue _aslife_ennemy)
      (set `self.Current Health` _returnvalue))))

(fn `UserConstructionScript`)
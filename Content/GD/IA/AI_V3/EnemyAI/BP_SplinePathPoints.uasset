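; BP_SplinePathPoints is an enemy AI actor that gathers the world-space points of its Spline01 component into a path array.
; On BeginPlay it loops over the spline points, appending each location to AllSplinePathPoints01.
; Debug code marked for deletion spawns small cubes and prints locations, re-walking the whole growing array after each append, so earlier points repeat.
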(event `self.ReceiveBeginPlay`
  (bind _spline01 (`self.Spline01`))
  (bind _allsplinepathpoints01 (`self.AllSplinePathPoints01`))
  (for _index (range (`SplineComponent.GetNumberOfSplinePoints` _spline01))
    (`KismetArrayLibrary.Array_Add` _allsplinepathpoints01 (`SplineComponent.GetLocationAtSplinePoint` _spline01 _index "World"))
    (for _array_element _allsplinepathpoints01
      ;[1 0.4179 0.4179] Delete
      (`|SpawnActorFromClass` "/Game/Blueprints/BP_CubeSimple_Delete.BP_CubeSimple_Delete_C" (`KismetMathLibrary.MakeTransform` _array_element (struct) (`KismetMathLibrary.MakeVector` 0.1 0.1 0.1)) "Undefined" "OverrideRootScale" null null)
      (`KismetSystemLibrary.PrintString` (`KismetStringLibrary.Conv_VectorToString` _array_element)))))

(fn `UserConstructionScript`)
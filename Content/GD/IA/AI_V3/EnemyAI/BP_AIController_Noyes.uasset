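; AI controller for Noyes enemies that runs the BT_AI_Enemy_Noyes behavior tree and caches the player character.
; Perception updates print the sense and store the player in the Blackboard.
; SeenPlayer and LostPlayer events set or clear the target and change guard walk speed; AttackZ forwards to the guard.
; HandleSense maps sight and hearing to investigation keys, but its only call is disconnected, as is the distance-based detection-speed logic.
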(event `self.ReceiveBeginPlay`
  (`self.RunBehaviorTree` "/Game/GD/IA/AI_V3/EnemyAI/BT_AI_Enemy_Noyes.BT_AI_Enemy_Noyes")
  (bind _asbp_noyes_character (cast `/Game/GD/BP_Controller_GameMode_MainCharacter_GameInstance/BP_Noyes_Character` (`GameplayStatics.GetPlayerCharacter` 0)))
  (set `self.Player` _asbp_noyes_character))

(event `self.AIPerception.OnTargetPerceptionUpdated`
  (params (Actor :type "Actor Object Reference") (Stimulus :type "AIStimulus Structure"))
  (bind _returnvalue (`AIPerceptionSystem.GetSenseClassForStimulus` Stimulus))
  (`KismetSystemLibrary.PrintString` (`KismetSystemLibrary.GetClassDisplayName` _returnvalue))
  (if (== Actor (`self.Player`))
    (`BlackboardComponent.SetValueAsObject` (`self.Blackboard`) "Player" (`self.Player`))))

(event `SeenPlayer`
  (`BlackboardComponent.SetValueAsObject` (`self.Blackboard`) "TargetLocationActor" (`GameplayStatics.GetPlayerCharacter` 0))
  (set `CharacterMovementComponent.MaxWalkSpeed` 200.0 (`Character.CharacterMovement` (`self.As Guard Enemy`))))

(event `LostPlayer`
  (`BlackboardComponent.SetValueAsObject` (`self.Blackboard`) "TargetLocationActor" null)
  (set `CharacterMovementComponent.MaxWalkSpeed` 150.0 (`Character.CharacterMovement` (`self.As Guard Enemy`)))
  (`BlackboardComponent.SetValueAsBool` (`self.Blackboard`) "IsInvestigating" false))

(event `AttackZ`
  (`/Game/GD/IA/AI_V3/EnemyAI/BP_AI_Characters_Deprecated/Deprecated_BP_AI_Main_Character.AttackZ` (`self.As Guard Enemy`)))

(fn `HandleSense`
  (params (Selection :type String) (SensedActor :type "Actor Object Reference") (Stimulus :type "AIStimulus Structure"))
  (bind (_stimulus_age _stimulus_expirationage _stimulus_strength _stimulus_stimuluslocation) (break `AIStimulus` (`local.Stimulus`)))
  (bind (_stimulus_age_2 _stimulus_expirationage_2 _stimulus_strength_2 _stimulus_stimuluslocation_2 _stimulus_receiverlocation _stimulus_tag _stimulus_bsuccessfullysensed) (break `AIStimulus` (`local.Stimulus`)))
  (bind (_stimulus_age_3 _stimulus_expirationage_3 _stimulus_strength_3 _stimulus_stimuluslocation_3 _stimulus_receiverlocation_2 _stimulus_tag_2 _stimulus_bsuccessfullysensed_2) (break `AIStimulus` (`local.Stimulus`)))
  (bind (_stimulus_age_4 _stimulus_expirationage_4 _stimulus_strength_4 _stimulus_stimuluslocation_4) (break `AIStimulus` (`local.Stimulus`)))
  (switch `string` Selection
    (:`AiSense_Sight`
      (`BlackboardComponent.SetValueAsBool` (`self.Blackboard`) "IsInvestigating" _stimulus_bsuccessfullysensed_2)
      (if _stimulus_bsuccessfullysensed_2
        ;[1 1 1] Alert Phase
        (if (== (`local.SensedActor`) (`GameplayStatics.GetPlayerCharacter` 0))
          (`BlackboardComponent.SetValueAsObject` (`self.Blackboard`) "TargetLocationActor" (`local.SensedActor`))
          (bind _ascharacter (cast `Character` (`self.K2_GetPawn`)))
          (set `CharacterMovementComponent.MaxWalkSpeed` 50.0 (`Character.CharacterMovement` _ascharacter)))
        (else
          (`BlackboardComponent.SetValueAsVector` (`self.Blackboard`) "TargetLocationVector" _stimulus_stimuluslocation)
          (`BlackboardComponent.SetValueAsObject` (`self.Blackboard`) "TargetLocationActor" null))))
    (:`AiSense_Hearing`
      (`BlackboardComponent.SetValueAsBool` (`self.Blackboard`) "IsInvestigating" _stimulus_bsuccessfullysensed)
      (`BlackboardComponent.SetValueAsVector` (`self.Blackboard`) "TargetLocationVector" _stimulus_stimuluslocation_4))))

(fn `UserConstructionScript`)
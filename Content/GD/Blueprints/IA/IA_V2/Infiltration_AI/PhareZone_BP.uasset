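; PhareZone_BP is a spotlight zone, apparently for infiltration detection, that cycles the light and its IsActive flag on and off.
; Chained Delays on Tick drive the cycle, switching off after 10 seconds and back on 5 seconds later.
; A Box overlap by the player while active casts to BP_Noyes_Character but does nothing further.
; The Detection function, holding only a retriggerable delay, is unused.
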(event `self.ReceiveTick`
  (params (DeltaSeconds :type "Float (single-precision)"))
  (`KismetSystemLibrary.Delay` 10.0)
  (`SceneComponent.SetVisibility` (`self.SpotLight`) false false)
  (set `self.IsActive` false)
  (`KismetSystemLibrary.Delay` 5.0)
  (`SceneComponent.SetVisibility` (`self.SpotLight`) true false)
  (set `self.IsActive` true))

(event `self.Box.OnComponentBeginOverlap`
  (params (OverlappedComponent :type "PrimitiveComponent Object Reference") (OtherActor :type "Actor Object Reference") (OtherComp :type "PrimitiveComponent Object Reference") (OtherBodyIndex :type Integer) (bFromSweep :type Boolean) (SweepResult :type "HitResult Structure (by ref)"))
  (bind _returnvalue (`GameplayStatics.GetPlayerCharacter` 0))
  (if (== OtherActor _returnvalue)
    (if (`self.IsActive`)
      (bind _asbp_third_person_character_moons (cast `/Game/GD/BP_Controller_GameMode_MainCharacter_GameInstance/BP_Noyes_Character` _returnvalue)))))

(event `self.Box.OnComponentHit`
  (params (HitComponent :type "PrimitiveComponent Object Reference") (OtherActor :type "Actor Object Reference") (OtherComp :type "PrimitiveComponent Object Reference") (NormalImpulse :type "Vector Structure") (Hit :type "HitResult Structure (by ref)")))

(fn `UserConstructionScript`)
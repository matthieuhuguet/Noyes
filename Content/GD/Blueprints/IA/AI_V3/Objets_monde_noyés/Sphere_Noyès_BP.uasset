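; Sphere actor for the "Noyés" (drowned) world mechanic, present only while that world is inactive.
; Every Tick polls the MondeNoyés flag, hiding the actor and disabling Sphere collision when true, otherwise showing it with query and physics collision.
; It starts visible on BeginPlay and reapplies its state each frame rather than only on changes.
; Nothing in this Blueprint sets the flag.
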(event `self.ReceiveBeginPlay`
  (`self.Appear`))

(event `Appear`
  (`self.SetActorHiddenInGame` false)
  (`PrimitiveComponent.SetCollisionEnabled` (`self.Sphere`) "QueryAndPhysics"))

(event `Disappear`
  (`self.SetActorHiddenInGame` true)
  (`PrimitiveComponent.SetCollisionEnabled` (`self.Sphere`) "NoCollision"))

(event `self.ReceiveTick`
  (params (DeltaSeconds :type "Float (single-precision)"))
  (if (`self.Monde Noyés?`)
    (`self.Disappear`)
    (else
      (`self.Appear`))))

(fn `UserConstructionScript`
  (`parent.UserConstructionScript`))
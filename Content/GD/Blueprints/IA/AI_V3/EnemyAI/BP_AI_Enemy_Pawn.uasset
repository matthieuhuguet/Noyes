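; Enemy AI character that reacts to damage with knockback, a hit montage and a life bar update.
; On any damage, it lowers its health and the Life_Ennemy widget value, launches along the player's facing direction, then plays a random montage from its list.
; Health only decreases when that widget is valid, and no death handling is present here.
; BeginPlay links the unarmed animation layers to the mesh.
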(event `self.ReceiveAnyDamage`
  (params (Damage :type "Float (single-precision)") (DamageType :type "DamageType Object Reference") (InstigatedBy :type "Controller Object Reference") (DamageCauser :type "Actor Object Reference"))
  (bind _anim_montage_ennemy (`self.Anim Montage Ennemy`))
  (`self.UpdateLifeWidget` Damage)
  (bind _asbp_third_person_character_moons (cast `/Game/ThirdPerson/Blueprints/BP_ThirdPersonCharacter_Moons` (`GameplayStatics.GetPlayerCharacter` 0)))
  (`self.LaunchCharacter` (* (`KismetMathLibrary.GetForwardVector` (`self.K2_GetActorRotation` _asbp_third_person_character_moons)) 1500.0))
  (`self.PlayAnimMontage` (`|GetArrayItem` _anim_montage_ennemy (`KismetMathLibrary.RandomIntegerInRange` 0 (- (`KismetArrayLibrary.Array_Length` _anim_montage_ennemy) 1)))))

(event `self.ReceiveBeginPlay`
  (`SkeletalMeshComponent.LinkAnimClassLayers` (`self.Mesh`) "/Game/GD/Characters/Heroes/Mannequin/Animations/Locomotion/Unarmed/ABP_UnarmedAnimLayers.ABP_UnarmedAnimLayers_C"))

(fn `UpdateLifeWidget`
  (params (DamageRecipient :type "Float (double-precision)"))
  (bind _returnvalue (- (`self.Current Health`) DamageRecipient))
  (bind _aslife_ennemy (cast `/Game/GD/UI_HUD/Life_Ennemy` (`WidgetComponent.GetUserWidgetObject` (`self.Widget`))))
  (`/Engine/EditorBlueprintResources/StandardMacros.IsValid` _aslife_ennemy
    (:`Is Valid`
      (set `/Game/GD/UI_HUD/Life_Ennemy.CurrentLifeUI` _returnvalue _aslife_ennemy)
      (set `self.Current Health` _returnvalue))))

(fn `UserConstructionScript`)
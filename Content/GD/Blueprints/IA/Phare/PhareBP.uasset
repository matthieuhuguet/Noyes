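; Lighthouse actor whose rotating light stops while a BP_Noyes_Character is inside its detection box.
; Tick plays a timeline that drives the light's yaw at a fixed pitch, or stops it while the InRange flag is set.
; Box overlap events set and clear that flag, printing a debug message on detection.
; A persistent debug line trace from the light to SphereEnd runs once at BeginPlay, with its result unused.
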(event `self.ReceiveBeginPlay`
  (bind _outhit (`KismetSystemLibrary.LineTraceSingle` :`Start` (`SceneComponent.K2_GetComponentLocation` (`self.Light`)) :`End` (`SceneComponent.K2_GetComponentLocation` (`self.SphereEnd`)) :`TraceChannel` "TraceTypeQuery1" :`DrawDebugType` "Persistent")))

(event `Rotation`
  (bind (_direction _newtrack_0) (`Timeline|Timeline_0` :!label _label)
    (:`Update`
      (`SceneComponent.K2_SetWorldRotation` (`self.Light`) (`KismetMathLibrary.MakeRotator` 0.0 20.0 _newtrack_0) false false))))

(event `self.ReceiveTick`
  (params (DeltaSeconds :type "Float (single-precision)"))
  (if (`self.InRange`)
    (goto _label :!via `Stop`)
    (else
      (`self.Rotation`))))

(event `self.Box.OnComponentBeginOverlap`
  (params (OverlappedComponent :type "PrimitiveComponent Object Reference") (OtherActor :type "Actor Object Reference") (OtherComp :type "PrimitiveComponent Object Reference") (OtherBodyIndex :type Integer) (bFromSweep :type Boolean) (SweepResult :type "HitResult Structure (by ref)"))
  (cast `/Game/GD/BP_Controller_GameMode_MainCharacter_GameInstance/BP_Noyes_Character` OtherActor)
  (set `self.InRange` true)
  (`KismetSystemLibrary.PrintString` "Detected" true true (struct :`R` 1.0 :`B` 0.101925 :`A` 1.0)))

(event `self.Box.OnComponentEndOverlap`
  (params (OverlappedComponent :type "PrimitiveComponent Object Reference") (OtherActor :type "Actor Object Reference") (OtherComp :type "PrimitiveComponent Object Reference") (OtherBodyIndex :type Integer))
  (cast `/Game/GD/BP_Controller_GameMode_MainCharacter_GameInstance/BP_Noyes_Character` OtherActor)
  (set `self.InRange` false))

(fn `UserConstructionScript`)
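; TB_Tonneau is a tutorial trigger that shows a French hint telling the player to press E to break barrels.
; Overlap with BP_Noyes_Character creates an Info_UI widget, and leaving removes it, with DoOnce gates that reset after a short delay.
; Tick polls the player's AmmoReserve, then destroys the trigger and removes the hint once any ammo is held.
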(event `self.ReceiveTick`
  (params (DeltaSeconds :type "Float (single-precision)"))
  (bind _noyescharacter (`/Game/GD/Blueprints_Function_Library/BFL_Player.Get Player Character`))
  (if (>= (`/Game/GD/BP_Controller_GameMode_MainCharacter_GameInstance/BP_Noyes_Character.Ammo Reserve` _noyescharacter) 1)
    (`self.K2_DestroyActor`)
    (`/Game/GD/UI_HUD/Mounir_WIP/Collectibles/Info_UI.Remove` (`self.InfoUI`))))

(event `self.CollisionComponent.OnComponentBeginOverlap`
  (params (OverlappedComponent :type "PrimitiveComponent Object Reference") (OtherActor :type "Actor Object Reference") (OtherComp :type "PrimitiveComponent Object Reference") (OtherBodyIndex :type Integer) (bFromSweep :type Boolean) (SweepResult :type "HitResult Structure (by ref)"))
  (cast `/Game/GD/BP_Controller_GameMode_MainCharacter_GameInstance/BP_Noyes_Character` OtherActor)
  (`/Engine/EditorBlueprintResources/StandardMacros.DoOnce` false :!label _label
    (:`Completed`
      (bind _returnvalue (`|CreateWidget` "/Game/GD/UI_HUD/Mounir_WIP/Collectibles/Info_UI.Info_UI_C"))
      (bind _output_get (set `self.InfoUI` _returnvalue))
      (set `/Game/GD/UI_HUD/Mounir_WIP/Collectibles/Info_UI.InfoText` "E pour casser des tonnneaux" _output_get)
      (`UserWidget.AddToViewport` _output_get 0))))

(event `self.CollisionComponent.OnComponentEndOverlap`
  (params (OverlappedComponent :type "PrimitiveComponent Object Reference") (OtherActor :type "Actor Object Reference") (OtherComp :type "PrimitiveComponent Object Reference") (OtherBodyIndex :type Integer))
  (cast `/Game/GD/BP_Controller_GameMode_MainCharacter_GameInstance/BP_Noyes_Character` OtherActor)
  (`/Engine/EditorBlueprintResources/StandardMacros.DoOnce` false :!label _label_2
    (:`Completed`
      (`/Game/GD/UI_HUD/Mounir_WIP/Collectibles/Info_UI.Remove` (`self.InfoUI`))
      (`KismetSystemLibrary.Delay` 0.5)
      (`|ExecutionSequence`
        (:`then_0`
          (goto _label :!via `Reset`))
        (:`then_1`
          (goto _label_2 :!via `Reset`))))))

(fn `UserConstructionScript`)
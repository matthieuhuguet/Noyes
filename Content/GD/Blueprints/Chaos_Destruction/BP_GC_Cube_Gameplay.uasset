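; BP_GC_Cube_Gameplay is a gameplay Geometry Collection cube that shatters through Chaos destruction when its break-cluster trigger fires.
; BeginPlay binds Break_Cluster to that trigger.
; The handler enables physics on the Geometry Collection, spawns a BP_MasterFieldProjectile at the actor's location and disables the Box collision.
; The Box overlap only casts to BP_Noyes_Character, and its BreakCluster call is left unconnected.
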(event `self.ReceiveBeginPlay`
  ;[1 1 1] This condition Break cluster
  (add `self.BreakClusterTrigger` (delegate `Break_Cluster`)))

(event `Break_Cluster`
  (bind _geometrycollectioncomponent (`self.GeometryCollectionComponent`))
  ;[1 1 1] This condition Break cluster
  (`/Engine/EditorBlueprintResources/StandardMacros.IsValid` _geometrycollectioncomponent
    (:`Is Valid`
      (`PrimitiveComponent.SetSimulatePhysics` _geometrycollectioncomponent true)
      (`|SpawnActorFromClass` "/Game/GD/Blueprints/Chaos_Destruction/BP_MasterFieldProjectile.BP_MasterFieldProjectile_C" (`KismetMathLibrary.MakeTransform` (`self.K2_GetActorLocation` self) (struct)) "Undefined" "OverrideRootScale" null null)
      (`PrimitiveComponent.SetCollisionProfileName` (`self.Box`) "NoCollision" true))))

(event `self.Box.OnComponentBeginOverlap`
  (params (OverlappedComponent :type "PrimitiveComponent Object Reference") (OtherActor :type "Actor Object Reference") (OtherComp :type "PrimitiveComponent Object Reference") (OtherBodyIndex :type Integer) (bFromSweep :type Boolean) (SweepResult :type "HitResult Structure (by ref)"))
  (cast `/Game/GD/BP_Controller_GameMode_MainCharacter_GameInstance/BP_Noyes_Character` OtherActor))

(fn `UserConstructionScript`)
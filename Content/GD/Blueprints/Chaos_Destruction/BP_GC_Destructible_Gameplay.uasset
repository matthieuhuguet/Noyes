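; Gameplay destructible Geometry Collection actor that breaks apart with a wood sound and drops an ammo box.
; The bound break-cluster trigger fires once, enabling physics simulation, destroying the capsule collision and spawning a master field projectile plus the scaled ammo pickup at the actor's location.
; In parallel, a timeline fades the debris material opacity to zero, then destroys the Geometry Collection component.
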(event `self.ReceiveBeginPlay`
  ;[1 1 1] This condition Break cluster
  (add `self.BreakClusterTrigger` (delegate `Break_Cluster`)))

(event `Break_Cluster`
  (bind _varspawnscale (`self.VarSpawnScale`))
  (bind _geometrycollectioncomponent (`self.GeometryCollectionComponent`))
  (bind _returnvalue (`self.K2_GetActorLocation` self))
  ;[1 1 1] This condition Break cluster
  (`/Engine/EditorBlueprintResources/StandardMacros.DoOnce` false
    (:`Completed`
      (`|ExecutionSequence`
        (:`then_0`
          (`/Engine/EditorBlueprintResources/StandardMacros.IsValid` _geometrycollectioncomponent
            (:`Is Valid`
              (`PrimitiveComponent.SetSimulatePhysics` _geometrycollectioncomponent true)
              (`ActorComponent.K2_DestroyComponent` (`self.CapsuleCollision`))
              (`GameplayStatics.PlaySound2D` "/Game/GD/Audio/Sounds/WoodBreak.WoodBreak" 1.0 1.0 0.0 null null)
              (`|SpawnActorFromClass` "/Game/GD/Blueprints/Chaos_Destruction/BP_MasterFieldProjectile.BP_MasterFieldProjectile_C" (`KismetMathLibrary.MakeTransform` _returnvalue) "Undefined" "OverrideRootScale" null null)
              (`|SpawnActorFromClass` "/Game/Environment_TA/Assets/Props/Munitions/BP_Boite_munition.BP_Boite_munition_C" (`KismetMathLibrary.MakeTransform` _returnvalue (struct :`Yaw` 90.0) (`KismetMathLibrary.MakeVector` _varspawnscale _varspawnscale _varspawnscale)) "Undefined" "OverrideRootScale" null null))))
        (:`then_1`
          (bind (_direction _alpha) (`Timeline|0-1` :!via `PlayFromStart`)
            (:`Update`
              (`MeshComponent.SetScalarParameterValueOnMaterials` (`self.GeometryCollectionComponent`) "Opacity" (`KismetMathLibrary.Lerp` 1.0 0.0 _alpha)))
            (:`Finished`
              (`ActorComponent.K2_DestroyComponent` (`self.GeometryCollectionComponent`)))))))))

(fn `UserConstructionScript`)
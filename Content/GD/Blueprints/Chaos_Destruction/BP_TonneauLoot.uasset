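; BP_TonneauLoot is a loot barrel that breaks apart on its own shortly after BeginPlay and drops an ammo box.
; After a delay, it spawns BP_Boite_munition at its location and swaps the intact mesh for a skeletal mesh playing a baked Alembic animation.
; After a further wait, a timeline fades the animated mesh through its Opacity material parameter, then destroys the actor.
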(event `self.ReceiveBeginPlay`
  (bind _tonneau_sk_anim (`self.Tonneau_SK_Anim`))
  ;[1 1 1] Declenchement BP
  (`KismetSystemLibrary.Delay` 2.0)
  (`self.Spawn_Munitions`)
  ;[1 1 1] T_Clean > T_SK_anim
  (`ActorComponent.K2_DestroyComponent` (`self.TonneauClean`))
  (`SceneComponent.SetVisibility` _tonneau_sk_anim true false)
  (`SkeletalMeshComponent.PlayAnimation` _tonneau_sk_anim "/Game/GD/Blueprints/Chaos_Destruction/Tonneau_Destruction/Tonneau_AlbAnim_Animation.Tonneau_AlbAnim_Animation" false)
  (`KismetSystemLibrary.Delay` (`self.WaitFadeDuration`))
  ;[1 1 1] Fade out
  (bind (_direction _newtrack_0) (`Timeline|Timeline_0`)
    (:`Update`
      (`MeshComponent.SetScalarParameterValueOnMaterials` (`self.Tonneau_SK_Anim`) "Opacity" (`KismetMathLibrary.Lerp` 1.0 0.0 _newtrack_0)))
    (:`Finished`
      (`self.K2_DestroyActor`))))

(event `Spawn_Munitions`
  (bind _var_spawn_scale (`self.Var Spawn Scale`))
  ;[0.3278 0.9216 1] Spawn Munitions
  (`|SpawnActorFromClass` "/Game/Environment_TA/Assets/Props/Munitions/BP_Boite_munition.BP_Boite_munition_C" (`KismetMathLibrary.MakeTransform` (`self.K2_GetActorLocation`) (struct :`Yaw` 90.0) (`KismetMathLibrary.MakeVector` _var_spawn_scale _var_spawn_scale _var_spawn_scale)) "Undefined" "OverrideRootScale" null null))

(fn `UserConstructionScript`)
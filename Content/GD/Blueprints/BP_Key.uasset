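; BP_Key is a key pickup that the player character, BP_Noyes_Character, collects by overlapping it.
; Its KeyNumber selects which flag is set on the character: Key1, Key2 or KeyEx.
; For a recognized number, the key then destroys itself and shows a UI_Item widget with the French "key obtained" message.
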(event `self.ReceiveActorBeginOverlap`
  (params (OtherActor :type "Actor Object Reference"))
  (bind _asbp_noyes_character (cast `/Game/GD/BP_Controller_GameMode_MainCharacter_GameInstance/BP_Noyes_Character` OtherActor))
  (if (== (`self.Key Number`) 0)
    (set `/Game/GD/BP_Controller_GameMode_MainCharacter_GameInstance/BP_Noyes_Character.Key 1` true _asbp_noyes_character)
    (`self.K2_DestroyActor` :!label _label)
    (bind _returnvalue (`|CreateWidget` "/Game/Environment_TA/Assets/Props/Munitions/UI_Item.UI_Item_C"))
    (set `/Game/Environment_TA/Assets/Props/Munitions/UI_Item.Got Item` "Clé Obtenue" _returnvalue)
    (`UserWidget.AddToViewport` _returnvalue 0)
    (elif (== (`self.Key Number`) 1)
      (set `/Game/GD/BP_Controller_GameMode_MainCharacter_GameInstance/BP_Noyes_Character.Key 2` true _asbp_noyes_character)
      (goto _label)
      (elif (== (`self.Key Number`) 2)
        (set `/Game/GD/BP_Controller_GameMode_MainCharacter_GameInstance/BP_Noyes_Character.Key Ex` true _asbp_noyes_character)
        (goto _label)))))

(fn `UserConstructionScript`)
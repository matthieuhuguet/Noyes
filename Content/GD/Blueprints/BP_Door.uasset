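; BP_Door is a key-gated swinging door that opens away from the player and can be closed again.
; OpenDoor requires HasKey, then plays or reverses a timeline that lerps the door's yaw, marking it closed once the reverse finishes.
; A dot product of the player-to-door direction and the door's forward vector picks the swing side.
; The construction script applies the configurable Mesh to the door.
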(event `self.ReceiveBeginPlay`
  (bind _asbp_noyes_character (cast `/Game/GD/BP_Controller_GameMode_MainCharacter_GameInstance/BP_Noyes_Character` (`GameplayStatics.GetPlayerCharacter` 0)))
  (set `self.Player Ref` _asbp_noyes_character))

(event `Open Door`
  (bind _defaultsceneroot (`self.DefaultSceneRoot`))
  (if (`self.HasKey`)
    (if (`self.IsDoorClosed`)
      (set `self.IsDoorClosed` false)
      (set `self.DotProduct` (`KismetMathLibrary.Dot_VectorVector` (`KismetMathLibrary.Normal` (- (`SceneComponent.K2_GetComponentLocation` _defaultsceneroot) (`self.K2_GetActorLocation` (`self.Player Ref`)))) (`SceneComponent.GetForwardVector` _defaultsceneroot)))
      (bind (_direction _alpha) (`Timeline|OpenDoorTL` :!label _label)
        (:`Update`
          (`SceneComponent.K2_SetRelativeRotation` (`self.Door`) (`KismetMathLibrary.MakeRotator` 0.0 0.0 (`KismetMathLibrary.Lerp` 0.0 (`KismetMathLibrary.SelectFloat` 90.0 -90.0 (>= (`self.DotProduct`) 0.0)) _alpha)) false false))
        (:`Finished`
          (switch `ETimelineDirection` _direction
            (:`Backward`
              (set `self.IsDoorClosed` true)))))
      (else
        (goto _label :!via `Reverse`)))))

(fn `UserConstructionScript`
  (`StaticMeshComponent.SetStaticMesh` (`self.Door`) (`self.Mesh`)))
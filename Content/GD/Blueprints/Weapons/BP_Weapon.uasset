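; BP_Weapon is a rifle weapon that attaches itself to the player's hand when touched.
; A Sphere overlap casts the other actor to Deprecated_ThirdPersonQuentin, stores it and snap-attaches to its mesh at the right grip socket.
; GetWeaponSocket returns world-space transforms of named sockets on the Rifle component.
; The damage, enemy life and arm alpha functions are stubs returning empty or default values.
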(event `self.Sphere.OnComponentBeginOverlap`
  (params (OverlappedComponent :type "PrimitiveComponent Object Reference") (OtherActor :type "Actor Object Reference") (OtherComp :type "PrimitiveComponent Object Reference") (OtherBodyIndex :type Integer) (bFromSweep :type Boolean) (SweepResult :type "HitResult Structure (by ref)"))
  (bind _asthird_person_quentin (cast `/Game/ThirdPerson/Blueprints/old/Deprecated_ThirdPersonQuentin` OtherActor))
  (set `self.TPS_Character` _asthird_person_quentin)
  (`self.K2_AttachToComponent` self (`Character.Mesh` (`self.TPS_Character`)) "Grip_Point_r" "SnapToTarget" "SnapToTarget" "SnapToTarget" true))

(fn `DamagedActualActor`
  (returns (ActorDamaged :type "Actor Object Reference"))
  (return null))

(fn `GetAlphaOnOffForArm`
  (returns (AlphaParameter :type Boolean))
  (return false))

(fn `GetWeaponSocket`
  (params (SocketName :type Name))
  (returns (SocketTransform :type "Transform Structure"))
  (return (`SceneComponent.GetSocketTransform` (`self.Rifle`) SocketName "RTS_World")))

(fn `UpdateLifeEnnemy`
  (returns (Guard_EnemyLife :type "Float (double-precision)"))
  (return 0.0))

(fn `UserConstructionScript`)
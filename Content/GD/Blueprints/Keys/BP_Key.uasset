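; BP_Key is a collectible key that shows a French "F" pickup prompt while BP_Noyes_Character overlaps its box.
; A DoOnce, reset shortly after the overlap ends, guards creation of the prompt widget.
; Got_Key, with no caller in this graph, increments KeyNumber and sets the matching Key1–3 flag on KeyMaster actors.
; Inside that loop, a matched key also destroys itself and displays a "key obtained" widget.
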(event `self.Box.OnComponentBeginOverlap`
  (params (OverlappedComponent :type "PrimitiveComponent Object Reference") (OtherActor :type "Actor Object Reference") (OtherComp :type "PrimitiveComponent Object Reference") (OtherBodyIndex :type Integer) (bFromSweep :type Boolean) (SweepResult :type "HitResult Structure (by ref)"))
  (cast `/Game/GD/BP_Controller_GameMode_MainCharacter_GameInstance/BP_Noyes_Character` OtherActor)
  (`/Engine/EditorBlueprintResources/StandardMacros.DoOnce` false :!label _label
    (:`Completed`
      (bind _returnvalue (`|CreateWidget` "/Game/GD/UI_HUD/Mounir_WIP/Collectibles/Info_UI.Info_UI_C"))
      (set `self.InfoUI` _returnvalue)
      (set `/Game/GD/UI_HUD/Mounir_WIP/Collectibles/Info_UI.InfoText` "\"F\" pour ramasser" (`self.InfoUI`))
      (`UserWidget.AddToViewport` (`self.InfoUI`) 0))))

(event `self.Box.OnComponentEndOverlap`
  (params (OverlappedComponent :type "PrimitiveComponent Object Reference") (OtherActor :type "Actor Object Reference") (OtherComp :type "PrimitiveComponent Object Reference") (OtherBodyIndex :type Integer))
  (cast `/Game/GD/BP_Controller_GameMode_MainCharacter_GameInstance/BP_Noyes_Character` OtherActor)
  (`/Game/GD/UI_HUD/Mounir_WIP/Collectibles/Info_UI.Remove` (`self.InfoUI`))
  (`KismetSystemLibrary.Delay` 0.5)
  (goto _label :!via `Reset`))

(event `Got_Key`
  (set `self.Key Number` (+ (`self.Key Number`) 1))
  (bind _outactors (`GameplayStatics.GetAllActorsOfClass` "/Game/GD/Blueprints/KeyMaster.KeyMaster_C"))
  (for _array_element _outactors
    (if (== (`self.Key Number`) 1)
      (set `/Game/GD/Blueprints/KeyMaster.Key 1` true _array_element)
      (`self.K2_DestroyActor` :!label _label_2)
      (bind _returnvalue (`|CreateWidget` "/Game/GD/UI_Item.UI_Item_C"))
      (set `/Game/GD/UI_Item.Number` "Clé Obtenue" _returnvalue)
      (`UserWidget.AddToViewport` _returnvalue 0)
      (elif (== (`self.Key Number`) 2)
        (set `/Game/GD/Blueprints/KeyMaster.Key 2` true _array_element)
        (goto _label_2)
        (elif (== (`self.Key Number`) 3)
          (set `/Game/GD/Blueprints/KeyMaster.Key 3` true _array_element)
          (goto _label_2))))))

(fn `UserConstructionScript`)
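; Construction-script tool actor that procedurally builds a modular building of cubic meshes along an editable spline.
; Wall segments are spaced by mesh bounds along the spline and stacked to a set height, with pillars at spline points and base pieces along the bottom.
; An optional roof fills the spline's bounding-box grid, using a segment-intersection point-in-polygon test to keep tiles inside the outline.
; Point snapping and corner base pieces exist but never run.
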(fn `BaseShapeFuction`
  (params (BaseShapeAsset :type "StaticMesh Object Reference") (BaseShapeAngleAsset :type "StaticMesh Object Reference"))
  (bind _spline (`self.Spline`))
  (for _index (range (+ (`self.LoopByLengthCurve`) 1))
    (bind _returnvalue (* _index (`self.Lenght`)))
    (bind (_x _y) (`KismetMathLibrary.BreakVector3f` (`SplineComponent.GetLocationAtDistanceAlongSpline` _spline _returnvalue "Local")))
    (bind _returnvalue_2 (`AddComponent|NODE_AddStaticMeshComponent-6` :`RelativeTransform` (`KismetMathLibrary.MakeTransform` (`KismetMathLibrary.MakeVector` _x _y) (`SplineComponent.GetRotationAtDistanceAlongSpline` _spline _returnvalue "Local") (1.0 1.0 1.0))))
    (`StaticMeshComponent.SetStaticMesh` _returnvalue_2 BaseShapeAsset))
  (return))

(fn `DoIntersect`
  (params (P1 :type "Vector Structure") (Q1 :type "Vector Structure") (P2 :type "Vector Structure") (Q2 :type "Vector Structure"))
  (returns (Intersect :type Boolean))
  (locals (O1 :type Integer :default 0) (O2 :type Integer :default 0) (O3 :type Integer :default 0) (O4 :type Integer :default 0))
  (bind _orientation (`self.Orientation` P1 Q1 P2))
  (bind _output_get (set `local.O1` _orientation))
  (bind _orientation_2 (`self.Orientation` P1 Q1 Q2))
  (bind _output_get_2 (set `local.O2` _orientation_2))
  (bind _orientation_3 (`self.Orientation` P2 Q2 P1))
  (bind _output_get_3 (set `local.O3` _orientation_3))
  (bind _orientation_4 (`self.Orientation` P2 Q2 Q1))
  (bind _output_get_4 (set `local.O4` _orientation_4))
  (return (and (!= _output_get _output_get_2) (!= _output_get_3 _output_get_4))))

(fn `GetMinMaxPoint`
  (returns (MinPoint1 :type "Vector Structure") (MaxPoint1 :type "Vector Structure"))
  (locals (MinPoint :type "Vector Structure") (MaxPoint :type "Vector Structure"))
  (bind _spline (`self.Spline`))
  (bind _returnvalue (`SplineComponent.GetLocationAtSplinePoint` _spline 0 "Local"))
  (set `local.MinPoint` _returnvalue)
  (set `local.MaxPoint` _returnvalue)
  (for _index (range (`SplineComponent.GetNumberOfSplinePoints` _spline))
    (set `local.MinPoint` (`KismetMathLibrary.Vector_ComponentMin` (`KismetMathLibrary.Vector_ComponentMin` (`SplineComponent.GetLocationAtSplinePoint` _spline _index "Local") (`SplineComponent.GetLocationAtSplinePoint` _spline (+ _index 1) "Local")) (`local.MinPoint`)))
    (set `local.MaxPoint` (`KismetMathLibrary.Vector_ComponentMax` (`KismetMathLibrary.Vector_ComponentMax` (`SplineComponent.GetLocationAtSplinePoint` _spline _index "Local") (`SplineComponent.GetLocationAtSplinePoint` _spline (+ _index 1) "Local")) (`local.MaxPoint`))))
  (return (`local.MinPoint`) (`local.MaxPoint`)))

(fn `IsInside`
  (params (P :type "Vector Structure"))
  (returns (IsInside :type Boolean))
  (locals (Count :type Integer))
  (bind _spline (`self.Spline`))
  (bind _returnvalue (`SplineComponent.GetNumberOfSplinePoints` _spline))
  (for _index (range _returnvalue)
    (bind _intersect (`self.DoIntersect` P (+ (`self.Pmin`) (-100.0 0.0 0.0)) (`SplineComponent.GetLocationAtSplinePoint` _spline _index "Local") (`SplineComponent.GetLocationAtSplinePoint` _spline (mod (+ _index 1) _returnvalue) "Local")))
    (if _intersect
      (`/Engine/EditorBlueprintResources/StandardMacros.IncrementInt` (`local.Count`))))
  (return (!= (mod (`local.Count`) 2) 0)))

(fn `Orientation`
  (params (P :type "Vector Structure") (Q :type "Vector Structure") (R :type "Vector Structure"))
  (returns (orientation :type Integer))
  (bind (_x _y) (`KismetMathLibrary.BreakVector3f` P))
  (bind (_x_2 _y_2) (`KismetMathLibrary.BreakVector3f` Q))
  (bind (_x_3 _y_3) (`KismetMathLibrary.BreakVector3f` R))
  (bind _returnvalue (- (* (- _y_2 _y) (- _x_3 _x_2)) (* (- _x_2 _x) (- _y_3 _y_2))))
  (if (== _returnvalue 0.0)
    (return 0)
    (elif (> _returnvalue 0.0)
      (return 1)
      (else
        (return 2)))))

(fn `PillardFuction`
  (params (PillardAsset :type "StaticMesh Object Reference"))
  (bind _spline (`self.Spline`))
  (for _index (range (`SplineComponent.GetNumberOfSplinePoints` _spline))
    (for _index_2 (range (`self.Height`))
      (bind (_returnvalue_x _returnvalue_y) (`KismetMathLibrary.BreakVector` (`SplineComponent.GetLocationAtSplinePoint` _spline _index "Local")))
      (bind _returnvalue (`AddComponent|NODE_AddStaticMeshComponent-5` :`RelativeTransform` (`KismetMathLibrary.MakeTransform` (`KismetMathLibrary.MakeVector` _returnvalue_x _returnvalue_y (* _index_2 (`self.Lenght`))) (`SplineComponent.GetRotationAtSplinePoint` _spline _index "Local"))))
      (`StaticMeshComponent.SetStaticMesh` _returnvalue PillardAsset)))
  (return))

(fn `PointSnapping`
  (bind _spline (`self.Spline`))
  (bind _returnvalue (/ (`self.Lenght`) 2.0))
  (bind _returnvalue_2 (- (`SplineComponent.GetNumberOfSplinePoints` _spline) 1))
  (bind (_returnvalue_x _returnvalue_y) (`KismetMathLibrary.BreakVector` (`SplineComponent.GetLocationAtSplinePoint` _spline _returnvalue_2 "Local")))
  (`SplineComponent.SetLocationAtSplinePoint` _spline _returnvalue_2 (`KismetMathLibrary.MakeVector` (+ _returnvalue_x (`KismetMathLibrary.SelectInt` 0 100 (== (mod (`KismetMathLibrary.Round` (/ _returnvalue_x _returnvalue)) 2) 0))) (+ _returnvalue_y (`KismetMathLibrary.SelectInt` 0 100 (== (mod (`KismetMathLibrary.Round` (/ _returnvalue_y _returnvalue)) 2) 0)))) "Local" true)
  (return))

(fn `RoofGenerator`
  (params (TargetMesh :type "StaticMesh Object Reference"))
  (bind _lenght (`self.Lenght`))
  (bind (_pmin_x _pmin_y) (`KismetMathLibrary.BreakVector` (`self.Pmin`)))
  (bind _returnvalue (* (`self.Height`) _lenght))
  (bind (_returnvalue_x _returnvalue_y) (`KismetMathLibrary.BreakVector` (- (`self.Pmax`) (`self.Pmin`))))
  (bind (_minpoint1 _maxpoint1) (`self.GetMinMaxPoint`))
  (set `self.Pmin` _minpoint1)
  (set `self.Pmax` _maxpoint1)
  (for _index (range (`KismetMathLibrary.FFloor` (+ (/ _returnvalue_x _lenght) 0.1)))
    (for _index_2 (range (`KismetMathLibrary.FFloor` (+ (/ _returnvalue_y _lenght) 0.1)))
      (bind _returnvalue_2 (+ (* (`self.Lenght`) _index) _pmin_x))
      (bind _returnvalue_3 (+ (* (`self.Lenght`) _index_2) _pmin_y))
      (bind _isinside (`self.IsInside` (`KismetMathLibrary.MakeVector` _returnvalue_2 _returnvalue_3 _returnvalue)))
      (if _isinside
        (bind _returnvalue_4 (`AddComponent|NODE_AddStaticMeshComponent-3` :`RelativeTransform` (`KismetMathLibrary.MakeTransform` (`KismetMathLibrary.MakeVector` _returnvalue_2 _returnvalue_3 _returnvalue))))
        (`StaticMeshComponent.SetStaticMesh` _returnvalue_4 TargetMesh))))
  (return))

(fn `TypeOfCurve`
  (bind _spline (`self.Spline`))
  (bind _spline_2 (`self.Spline`))
  (for _index (range (+ (+ (`SplineComponent.GetNumberOfSplinePoints` _spline) 2) 1))
    (if (> (`SplineComponent.GetSplineLength` _spline_2) 201.0)
      (`SplineComponent.SetSplinePointType` _spline _index "Linear" true)
      (else
        (`SplineComponent.SetSplinePointType` _spline_2 _index "Curve" true))))
  (return))

(fn `UserConstructionScript`
  (locals (PointVecMin :type "Vector Structure") (PointVecMax :type "Vector Structure"))
  (bind _upwallasset (`self.UpWallAsset`))
  (bind _ground (`self.Ground`))
  (bind _baseasset (`self.BaseAsset`))
  (bind _pillard (`self.Pillard`))
  (bind _basegroundshape (`self.BaseGroundShape`))
  (bind _basegroundshapeangle (`self.BaseGroundShapeAngle`))
  (bind _output (`|GetArrayItem` _baseasset (`KismetMathLibrary.RandomIntegerInRange` 0 (- (`KismetArrayLibrary.Array_Length` _baseasset) 1))))
  (bind (_returnvalue_min _returnvalue_max) (break `Box` (`StaticMesh.GetBoundingBox` _output)))
  (bind _returnvalue_x (`KismetMathLibrary.BreakVector` (- _returnvalue_max _returnvalue_min)))
  (bind _returnvalue (+ _returnvalue_x (`self.Offset`)))
  (bind _returnvalue_2 (`KismetMathLibrary.FTrunc` (/ (`SplineComponent.GetSplineLength` (`self.Spline`)) _returnvalue)))
  (`self.TypeOfCurve`) ; Set linear or curve
  (`SplineComponent.SetClosedLoop` (`self.Spline`) (`self.In Closed Loop`) true)
  (set `self.Lenght` _returnvalue)
  (set `self.LoopByLengthCurve` _returnvalue_2)
  (`self.WallGeneration` _returnvalue_2 _output (`|GetArrayItem` _upwallasset (`KismetMathLibrary.RandomIntegerInRange` 0 (- (`KismetArrayLibrary.Array_Length` _upwallasset) 1))))
  (if (`self.Roof`)
    (`self.RoofGenerator` (`|GetArrayItem` _ground (`KismetMathLibrary.RandomIntegerInRange` 0 (- (`KismetArrayLibrary.Array_Length` _ground) 1)))))
  (`self.PillardFuction` (`|GetArrayItem` _pillard (`KismetMathLibrary.RandomIntegerInRange` 0 (- (`KismetArrayLibrary.Array_Length` _pillard) 1))))
  (`self.BaseShapeFuction` (`|GetArrayItem` _basegroundshape (`KismetMathLibrary.RandomIntegerInRange` 0 (- (`KismetArrayLibrary.Array_Length` _basegroundshape) 1))) (`|GetArrayItem` _basegroundshapeangle (`KismetMathLibrary.RandomIntegerInRange` 0 (- (`KismetArrayLibrary.Array_Length` _basegroundshapeangle) 1)))))

(fn `WallGeneration`
  (params (LastIndex :type Integer) (DownWallPart :type "StaticMesh Object Reference") (UpWallPart :type "StaticMesh Object Reference"))
  (bind _spline (`self.Spline`))
  (for _index (range (+ LastIndex 1))
    (for _index_2 (range (`self.Height`))
      (bind _returnvalue (* _index (`self.Lenght`)))
      (bind (_x _y) (`KismetMathLibrary.BreakVector3f` (`SplineComponent.GetLocationAtDistanceAlongSpline` _spline _returnvalue "Local")))
      (bind _returnvalue_2 (* (`self.Lenght`) _index_2))
      (bind _returnvalue_3 (`AddComponent|NODE_AddStaticMeshComponent-0` :`RelativeTransform` (`KismetMathLibrary.MakeTransform` (`KismetMathLibrary.MakeVector` _x _y _returnvalue_2) (`SplineComponent.GetRotationAtDistanceAlongSpline` _spline _returnvalue "Local") (`KismetMathLibrary.MakeVector` 1.0 (`KismetMathLibrary.SelectFloat` 1.0 -1.0 (`self.FlipFacing`)) 1.0))))
      (if (> _returnvalue_2 20.0)
        (`StaticMeshComponent.SetStaticMesh` _returnvalue_3 DownWallPart)
        (else
          (`StaticMeshComponent.SetStaticMesh` _returnvalue_3 UpWallPart)))))
  (return))
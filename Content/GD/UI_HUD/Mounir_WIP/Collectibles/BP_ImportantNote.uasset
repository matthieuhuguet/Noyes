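; BP_ImportantNote is a collectible note actor whose text and image come from a data table.
; On BeginPlay it looks up its RowName in Notes_DataTable and stores that row's text and image.
; The construction script applies the NoteModel mesh to the Model component, and DestroyAction removes the actor.
; GetText returns an empty string rather than the loaded text.
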(event `/Game/GD/BI_Interfaces/BI_Interaction_Interface.DestroyAction`
  (`self.K2_DestroyActor`))

(event `self.ReceiveBeginPlay`
  (bind _returnvalue (`|GetDataTableRow` "/Game/GD/UI_HUD/Mounir_WIP/Collectibles/Notes_DataTable.Notes_DataTable" (`self.Row Name`))
    (:`then`
      (bind (_location _number _keynote_ _image _texte) (break `/Game/GD/UI_HUD/Mounir_WIP/Collectibles/Notes_Stru` _returnvalue))
      (set `self.Text` _texte)
      (set `self.2d Image` _image))))

(fn `GetText`
  (returns (TextString :type Text))
  (return ""))

(fn `UserConstructionScript`
  (`StaticMeshComponent.SetStaticMesh` (`self.Model`) (`self.Note Model`)))
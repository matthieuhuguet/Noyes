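; Collectible small note actor that prompts the player to read it when nearby and stores the note's content.
; BeginPlay loads its text and image from a Notes data table row, and the construction script applies its mesh.
; Box overlaps with BP_Noyes_Character add and remove an "F pour lire" widget, gated by DoOnce nodes that reset after a short delay on exit.
; Reading is not handled here; DestroyAction destroys the actor and GetText returns empty.
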(event `/Game/GD/BI_Interfaces/BI_Interaction_Interface.DestroyAction`
  (`self.K2_DestroyActor`))

(event `self.ReceiveBeginPlay`
  (bind _returnvalue (`|GetDataTableRow` "/Game/GD/UI_HUD/Mounir_WIP/Collectibles/Notes_DataTable.Notes_DataTable" (`self.Row Name`))
    (:`then`
      (bind (_location _number _keynote_ _image _texte) (break `/Game/GD/UI_HUD/Mounir_WIP/Collectibles/Notes_Stru` _returnvalue))
      (set `self.Text` _texte)
      (set `self.2d Image` _image))))

(event `self.Box.OnComponentBeginOverlap`
  (params (OverlappedComponent :type "PrimitiveComponent Object Reference") (OtherActor :type "Actor Object Reference") (OtherComp :type "PrimitiveComponent Object Reference") (OtherBodyIndex :type Integer) (bFromSweep :type Boolean) (SweepResult :type "HitResult Structure (by ref)"))
  (cast `/Game/GD/BP_Controller_GameMode_MainCharacter_GameInstance/BP_Noyes_Character` OtherActor)
  (`/Engine/EditorBlueprintResources/StandardMacros.DoOnce` false :!label _label
    (:`Completed`
      (bind _returnvalue (`|CreateWidget` "/Game/GD/UI_HUD/Mounir_WIP/Collectibles/Info_UI.Info_UI_C"))
      (bind _output_get (set `self.InfoUI` _returnvalue))
      (set `/Game/GD/UI_HUD/Mounir_WIP/Collectibles/Info_UI.InfoText` "F pour lire" _output_get)
      (`UserWidget.AddToViewport` _output_get 0))))

(event `self.Box.OnComponentEndOverlap`
  (params (OverlappedComponent :type "PrimitiveComponent Object Reference") (OtherActor :type "Actor Object Reference") (OtherComp :type "PrimitiveComponent Object Reference") (OtherBodyIndex :type Integer))
  (cast `/Game/GD/BP_Controller_GameMode_MainCharacter_GameInstance/BP_Noyes_Character` OtherActor)
  (`/Engine/EditorBlueprintResources/StandardMacros.DoOnce` false :!label _label_2
    (:`Completed`
      (`/Game/GD/UI_HUD/Mounir_WIP/Collectibles/Info_UI.Remove` (`self.InfoUI`))
      (`KismetSystemLibrary.Delay` 0.5)
      (`|ExecutionSequence`
        (:`then_0`
          (goto _label :!via `Reset`))
        (:`then_1`
          (goto _label_2 :!via `Reset`))))))

(fn `GetText`
  (returns (TextString :type Text))
  (return ""))

(fn `UserConstructionScript`
  (`StaticMeshComponent.SetStaticMesh` (`self.Model`) (`self.Note Model`)))
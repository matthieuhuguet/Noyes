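; AC_MERGING_CODE appears to be a scratch component holding code to merge into the character, with no active logic.
; AttackAI and the helper functions for rifle animation and smoke FX are empty.
; Two disconnected fragments hold an empty-rifle shot (sound, animation, smoke, retriggerable cooldown) and a forward sphere trace that plays a sound on hitting BP_Noyes_Character.
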(event `AttackAI`
  ;[1 1 1] Working Fine To Damaging AICharacter + Set Widget Hidden
)

(fn `PlayAnimationRifle`)

(fn `SpawnFXSmoke`
  (params (InSocketName :type Name) (Scale :type "Vector Structure")))
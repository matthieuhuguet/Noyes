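; HUD Blueprint that creates the game's main UI widgets and exposes events to show them.
; On BeginPlay it adds UMG_All as the first layer, then creates the journal, loading screen and startup menu and adds them from an array.
; The AI detection flash widget is created but never added to the viewport here.
; Display events set widgets visible; only UMG_All has a hide event, and DisplayOptions is empty.
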(event `self.ReceiveBeginPlay`
  ;[1 0.5647 1] Create Main Widget First Layer is added to viewport.
  (bind _returnvalue (`|CreateWidget` "/Game/GD/UI_HUD/UMG_All.UMG_All_C"))
  (bind _output_get (set `self.UMG_All_Object` _returnvalue))
  (`UserWidget.AddToViewport` _output_get 0)
  ;[0.5089 0.4452 1] Create Sub Widgets
  (bind _returnvalue_2 (`|CreateWidget` "/Game/GD/UI_HUD/WBP_FlashWhenDetected_AI.WBP_FlashWhenDetected_AI_C"))
  (set `self.WBP_FlashWhenDetectedAI` _returnvalue_2)
  (bind _returnvalue_3 (`|CreateWidget` "/Game/GD/UI_HUD/Mounir_WIP/Journal/Journal_BP.Journal_BP_C"))
  (bind _output_get_2 (set `self.JournalWidget` _returnvalue_3))
  (`KismetArrayLibrary.Array_Add` (`self.WBP_WidgetsCreated`) _output_get_2)
  (bind _returnvalue_4 (`|CreateWidget` "/Game/GD/UI_HUD/UI_Widgets_Menu/Menu/Loading_Screen.Loading_Screen_C"))
  (bind _output_get_3 (set `self.WBP_LoadingScreen` _returnvalue_4))
  (`KismetArrayLibrary.Array_Add` (`self.WBP_WidgetsCreated`) _output_get_3)
  (bind _returnvalue_5 (`|CreateWidget` "/Game/GD/UI_HUD/UI_Widgets_Menu/Menu/Startup_Menu.Startup_Menu_C"))
  (bind _output_get_4 (set `self.WBP_StartupMenu` _returnvalue_5))
  (`KismetArrayLibrary.Array_Add` (`self.WBP_WidgetsCreated`) _output_get_4)
  (for _array_element (`self.WBP_WidgetsCreated`)
    (`UserWidget.AddToViewport` _array_element 0)))

(event `DisplayWBPFlash`
  ;[0.5089 0.4452 1] Flash Logic For AI Widget
  (`Widget.SetVisibility` (`self.WBP_FlashWhenDetectedAI`) "Visible"))

(event `DisplayWBP_UMG_All`
  ;[0.5906 1 0.521] On
  (`Widget.SetVisibility` (`self.UMG_All_Object`) "Visible"))

(event `Hide_WBP_UMG_ALL`
  ;[1 0.4179 0.4179] Off
  (`Widget.SetVisibility` (`self.UMG_All_Object`) "Collapsed"))

(event `DisplayWBPJournal`
  (`Widget.SetVisibility` (`self.JournalWidget`) "Visible"))

(event `DisplayWBPLoadingScreen`
  (`Widget.SetVisibility` (`self.WBP_LoadingScreen`) "Visible"))

(event `Display_Startup_Menu`
  (`self.SetWidgetVisible` (`self.WBP_StartupMenu`)))

(event `Display Options`)

(fn `SetWidgetVisible`
  (params (Target :type "Widget Object Reference") (InVisibility :type "ESlateVisibility Enum" :default "Visible"))
  (`Widget.SetVisibility` Target InVisibility))

(fn `UserConstructionScript`)
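; Jean NPC character Blueprint that handles the character's dialogue text once its dialogue has been read.
; Tick checks HasReadDialogue and, while it is true, calls the new-text event every frame.
; The New_Text event writes the first two NPCText entries back into their own slots, so as shown the text stays unchanged.
; The construction script only runs the parent's.
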(event `self.ReceiveTick`
  (params (DeltaSeconds :type "Float (single-precision)"))
  (if (`self.Has Read Dialogue`)
    (`self.New_Text`)))

(event `New_Text`
  (bind _npc_text (`self.NPC_Text`))
  (`KismetArrayLibrary.Array_Set` _npc_text 0 (`|GetArrayItem` _npc_text))
  (`KismetArrayLibrary.Array_Set` _npc_text 1 (`|GetArrayItem` _npc_text 1)))

(fn `UserConstructionScript`
  (`parent.UserConstructionScript`))
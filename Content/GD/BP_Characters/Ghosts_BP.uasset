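; Ghost NPC Blueprint that offers text dialogue when BP_Noyes_Character enters its Box trigger.
; Box overlap adds a Dialogue_Box widget to the viewport, and end overlap removes that initially created widget, both printing debug messages.
; ActivateDialogue passes NPCText to the widget, reveals it and advances TextRow, replacing the widget with a fresh one at the last row.
; A DoOnce gates each activation and is reset after the step.
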(event `self.Box.OnComponentBeginOverlap`
  (params (OverlappedComponent :type "PrimitiveComponent Object Reference") (OtherActor :type "Actor Object Reference") (OtherComp :type "PrimitiveComponent Object Reference") (OtherBodyIndex :type Integer) (bFromSweep :type Boolean) (SweepResult :type "HitResult Structure (by ref)"))
  ;[1 1 1] Show Interact
  (cast `/Game/GD/BP_Controller_GameMode_MainCharacter_GameInstance/BP_Noyes_Character` OtherActor)
  (`KismetSystemLibrary.PrintString` "Talk to me" true true (struct :`R` 1.0 :`B` 0.020607 :`A` 1.0) 10.0)
  (bind _returnvalue (`|CreateWidget` "/Game/GD/UI_HUD/Mounir_WIP/Dialogue/Dialogue_Box.Dialogue_Box_C"))
  (bind _output_get (set `self.DialogueBox` _returnvalue))
  (`UserWidget.AddToViewport` _output_get 0))

(event `self.Box.OnComponentEndOverlap`
  (params (OverlappedComponent :type "PrimitiveComponent Object Reference") (OtherActor :type "Actor Object Reference") (OtherComp :type "PrimitiveComponent Object Reference") (OtherBodyIndex :type Integer))
  ;[1 1 1] Show Interact
  (cast `/Game/GD/BP_Controller_GameMode_MainCharacter_GameInstance/BP_Noyes_Character` OtherActor)
  (`Widget.RemoveFromParent` (stale `self.Box.OnComponentBeginOverlap` _returnvalue))
  (`KismetSystemLibrary.PrintString` "See ya" true true (struct :`R` 1.0 :`B` 0.020607 :`A` 1.0) 10.0))

(event `/Game/GD/BI_Interfaces/NPC_Interact.Activate Dialogue`
  (bind _dialoguebox (`self.DialogueBox`))
  (bind _returnvalue (+ (`/Game/GD/UI_HUD/Mounir_WIP/Dialogue/Dialogue_Box.TextRow` (`self.DialogueBox`)) 1))
  (`/Engine/EditorBlueprintResources/StandardMacros.DoOnce` false :!label _label
    (:`Completed`
      (set `/Game/GD/UI_HUD/Mounir_WIP/Dialogue/Dialogue_Box.Text` (`self.NPC_Text`) _dialoguebox)
      (`Widget.SetVisibility` (`/Game/GD/UI_HUD/Mounir_WIP/Dialogue/Dialogue_Box.TextBlock_0` _dialoguebox) "Visible")
      (`Widget.SetVisibility` (`/Game/GD/UI_HUD/Mounir_WIP/Dialogue/Dialogue_Box.Image_0` _dialoguebox) "Visible")
      (if (> _returnvalue (- (`KismetArrayLibrary.Array_Length` (`self.NPC_Text`)) 1))
        (`Widget.RemoveFromParent` (`self.DialogueBox`))
        (`self.Reset Dialogue`)
        (`self.Create Box`)
        (else
          (set `/Game/GD/UI_HUD/Mounir_WIP/Dialogue/Dialogue_Box.TextRow` _returnvalue (`self.DialogueBox`))
          (`self.Reset Dialogue`))))))

(event `Reset Dialogue`
  (goto _label :!via `Reset`))

(event `Create Box`
  (bind _returnvalue (`|CreateWidget` "/Game/GD/UI_HUD/Mounir_WIP/Dialogue/Dialogue_Box.Dialogue_Box_C"))
  (bind _output_get (set `self.DialogueBox` _returnvalue))
  (`UserWidget.AddToViewport` _output_get 0))

(fn `UserConstructionScript`)
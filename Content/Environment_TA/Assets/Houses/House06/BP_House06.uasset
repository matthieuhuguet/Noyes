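; BP_House06 is a configurable house environment Blueprint with optional shutters, foundations and barriers.
; Its construction script uses three booleans (Volets, Fondation, Barrieres) to show or hide the matching components.
; Dynamic material logic for facade color, detail brightness, roof material and foundation color is present but disconnected, so it never runs.
; The event graph holds only disabled placeholder events, with no runtime behavior.
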(fn `UserConstructionScript`
  (bind _voletbas1d (`self.voletBas1D`))
  (bind _fondations (`self.Fondations`))
  (bind _barriere5 (`self.Barriere5`))
  (`|ExecutionSequence`
    (:`then_0`
      ;[1 1 1] Visibility
      (if (`self.Volets?`)
        (`SceneComponent.SetVisibility` _voletbas1d true false)
        (`SceneComponent.SetVisibility` (`self.voletBas2D`) true false)
        (`SceneComponent.SetVisibility` (`self.voletBas1G`) true false)
        (`SceneComponent.SetVisibility` (`self.voletBas2G`) true false)
        (`SceneComponent.SetVisibility` (`self.voletMid2D`) true false)
        (`SceneComponent.SetVisibility` (`self.voletMid2G`) true false)
        (`SceneComponent.SetVisibility` (`self.voletMid3G`) true false)
        (`SceneComponent.SetVisibility` (`self.voletMid3D`) true false)
        (`SceneComponent.SetVisibility` (`self.voletHaut2G`) true false)
        (`SceneComponent.SetVisibility` (`self.voletHaut2D`) true false)
        (`SceneComponent.SetVisibility` (`self.voletBas1G2`) true false)
        (`SceneComponent.SetVisibility` (`self.voletHaut2G1`) true false)
        (`SceneComponent.SetVisibility` (`self.voletHaut2D1`) true false)
        (`SceneComponent.SetVisibility` (`self.voletBas1G10`) true false)
        (`SceneComponent.SetVisibility` (`self.voletHaut2G2`) true false)
        (`SceneComponent.SetVisibility` (`self.voletHaut2D2`) true false)
        (`SceneComponent.SetVisibility` (`self.voletBas1G1`) true false)
        (`SceneComponent.SetVisibility` (`self.voletBas1G11`) true false)
        (`SceneComponent.SetVisibility` (`self.voletBas1G3`) true false)
        (`SceneComponent.SetVisibility` (`self.voletBas1G4`) true false)
        (`SceneComponent.SetVisibility` (`self.voletBas1G8`) true false)
        (`SceneComponent.SetVisibility` (`self.voletBas1G5`) true false)
        (`SceneComponent.SetVisibility` (`self.voletBas1G6`) true false)
        (`SceneComponent.SetVisibility` (`self.voletBas1G7`) true false)
        (else
          (`SceneComponent.SetVisibility` _voletbas1d false false)
          (`SceneComponent.SetVisibility` (`self.voletBas2D`) false false)
          (`SceneComponent.SetVisibility` (`self.voletBas1G`) false false)
          (`SceneComponent.SetVisibility` (`self.voletBas2G`) false false)
          (`SceneComponent.SetVisibility` (`self.voletMid2D`) false false)
          (`SceneComponent.SetVisibility` (`self.voletMid2G`) false false)
          (`SceneComponent.SetVisibility` (`self.voletMid3G`) false false)
          (`SceneComponent.SetVisibility` (`self.voletMid3D`) false false)
          (`SceneComponent.SetVisibility` (`self.voletHaut2G`) false false)
          (`SceneComponent.SetVisibility` (`self.voletHaut2D`) false false)
          (`SceneComponent.SetVisibility` (`self.voletBas1G2`) false false)
          (`SceneComponent.SetVisibility` (`self.voletHaut2G1`) false false)
          (`SceneComponent.SetVisibility` (`self.voletHaut2D1`) false false)
          (`SceneComponent.SetVisibility` (`self.voletBas1G10`) false false)
          (`SceneComponent.SetVisibility` (`self.voletHaut2G2`) false false)
          (`SceneComponent.SetVisibility` (`self.voletHaut2D2`) false false)
          (`SceneComponent.SetVisibility` (`self.voletBas1G1`) false false)
          (`SceneComponent.SetVisibility` (`self.voletBas1G11`) false false)
          (`SceneComponent.SetVisibility` (`self.voletBas1G3`) false false)
          (`SceneComponent.SetVisibility` (`self.voletBas1G4`) false false)
          (`SceneComponent.SetVisibility` (`self.voletBas1G8`) false false)
          (`SceneComponent.SetVisibility` (`self.voletBas1G5`) false false)
          (`SceneComponent.SetVisibility` (`self.voletBas1G6`) false false)
          (`SceneComponent.SetVisibility` (`self.voletBas1G7`) false false))))
    (:`then_1`
      (if (`self.Fondation?`)
        (`SceneComponent.SetVisibility` _fondations true false)
        (else
          (`SceneComponent.SetVisibility` _fondations false false))))
    (:`then_2`
      (if (`self.Barrieres?`)
        (`SceneComponent.SetVisibility` _barriere5 true false)
        (`SceneComponent.SetVisibility` (`self.Barriere2`) true false)
        (`SceneComponent.SetVisibility` (`self.Barriere4`) true false)
        (`SceneComponent.SetVisibility` (`self.Barriere1`) true false)
        (else
          (`SceneComponent.SetVisibility` _barriere5 false false)
          (`SceneComponent.SetVisibility` (`self.Barriere2`) false false)
          (`SceneComponent.SetVisibility` (`self.Barriere4`) false false)
          (`SceneComponent.SetVisibility` (`self.Barriere1`) false false))))))
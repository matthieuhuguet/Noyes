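; Configurable boutique house Blueprint for environment dressing, set up entirely in the Construction Script.
; Toggles show or hide the eight shutters, the foundation and the two railings.
; Upper and lower shutter yaws are either set manually or drawn from a random stream, with lower ones biased to either end of their swing and left sides mirroring right.
; Material logic for facade color, detail brightness and roof is present but disconnected.
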(fn `UserConstructionScript`
  (bind _random_stream (`self.Random Stream`))
  (bind _rotation_volets_bas (`self.rotation volets bas`))
  (bind _rotation_volets_haut (`self.rotation volets haut`))
  (bind _voletbas1d (`self.voletBas1D`))
  (bind _fondations (`self.Fondations`))
  (bind _barriere2 (`self.Barriere2`))
  (`|ExecutionSequence`
    (:`then_0`
      ;[1 1 1] Visibility
      (if (`self.Volets?`)
        (`SceneComponent.SetVisibility` _voletbas1d true false)
        (`SceneComponent.SetVisibility` (`self.voletBas2D`) true false)
        (`SceneComponent.SetVisibility` (`self.voletBas1G`) true false)
        (`SceneComponent.SetVisibility` (`self.voletBas2G`) true false)
        (`SceneComponent.SetVisibility` (`self.voletHaut2G`) true false)
        (`SceneComponent.SetVisibility` (`self.voletHaut2D`) true false)
        (`SceneComponent.SetVisibility` (`self.voletHaut1G`) true false)
        (`SceneComponent.SetVisibility` (`self.voletHaut1D`) true false)
        (if (`self.RotRandom`)
          ;[1 1 1] Rotation Random
          (`|ExecutionSequence`
            (:`then_0`
              (set `self.rotation volets bas` (`KismetMathLibrary.SelectFloat` (`KismetMathLibrary.RandomFloatInRangeFromStream` 0.0 30.0 _random_stream) (`KismetMathLibrary.RandomFloatInRangeFromStream` 150.0 180.0 _random_stream) (`KismetMathLibrary.RandomBool`))))
            (:`then_2`
              (set `self.rotation volets haut` (`KismetMathLibrary.RandomFloatInRangeFromStream` 30.0 180.0 _random_stream))
              ;[1 1 1] Rotation Variable
              (`|ExecutionSequence` :!label _label
                (:`then_0`
                  (`SceneComponent.K2_SetRelativeRotation` (`self.voletBas1D`) (`KismetMathLibrary.MakeRotator` 0.0 0.0 _rotation_volets_bas) false false)
                  (`SceneComponent.K2_SetRelativeRotation` (`self.voletBas2D`) (`KismetMathLibrary.MakeRotator` 0.0 0.0 _rotation_volets_bas) false false))
                (:`then_1`
                  (`SceneComponent.K2_SetRelativeRotation` (`self.voletBas1G`) (`KismetMathLibrary.MakeRotator` 0.0 0.0 (* _rotation_volets_bas -1.0)) false false)
                  (`SceneComponent.K2_SetRelativeRotation` (`self.voletBas2G`) (`KismetMathLibrary.MakeRotator` 0.0 0.0 (* _rotation_volets_bas -1.0)) false false))
                (:`then_4`
                  (`SceneComponent.K2_SetRelativeRotation` (`self.voletHaut2D`) (`KismetMathLibrary.MakeRotator` 0.0 0.0 _rotation_volets_haut) false false)
                  (`SceneComponent.K2_SetRelativeRotation` (`self.voletHaut1D`) (`KismetMathLibrary.MakeRotator` 0.0 0.0 _rotation_volets_haut) false false))
                (:`then_5`
                  (`SceneComponent.K2_SetRelativeRotation` (`self.voletHaut2G`) (`KismetMathLibrary.MakeRotator` 0.0 0.0 (* _rotation_volets_haut -1.0)) false false)
                  (`SceneComponent.K2_SetRelativeRotation` (`self.voletHaut1G`) (`KismetMathLibrary.MakeRotator` 0.0 0.0 (* _rotation_volets_haut -1.0)) false false)))))
          (else
            (goto _label)))
        (else
          (`SceneComponent.SetVisibility` _voletbas1d false false)
          (`SceneComponent.SetVisibility` (`self.voletBas2D`) false false)
          (`SceneComponent.SetVisibility` (`self.voletBas1G`) false false)
          (`SceneComponent.SetVisibility` (`self.voletBas2G`) false false)
          (`SceneComponent.SetVisibility` (`self.voletHaut2G`) false false)
          (`SceneComponent.SetVisibility` (`self.voletHaut2D`) false false)
          (`SceneComponent.SetVisibility` (`self.voletHaut1G`) false false)
          (`SceneComponent.SetVisibility` (`self.voletHaut1D`) false false))))
    (:`then_1`
      (if (`self.Fondation?`)
        (`SceneComponent.SetVisibility` _fondations true false)
        (else
          (`SceneComponent.SetVisibility` _fondations false false))))
    (:`then_2`
      (if (`self.Barrieres?`)
        (`SceneComponent.SetVisibility` _barriere2 true false)
        (`SceneComponent.SetVisibility` (`self.Barriere1`) true false)
        (else
          (`SceneComponent.SetVisibility` _barriere2 false false)
          (`SceneComponent.SetVisibility` (`self.Barriere1`) false false))))))
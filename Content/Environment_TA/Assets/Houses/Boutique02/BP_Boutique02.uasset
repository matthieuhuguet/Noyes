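; Configurable boutique house prop whose look is built entirely in the Construction Script from exposed variables.
; Toggles show or hide shutters, foundations, barriers and butcher, bookshop and hat-shop dressings.
; Shutter rows share a yaw, mirrored left to right, either set manually or randomised from a stream, though the bottom row's range choice uses an unseeded RandomBool.
; Dynamic material instances drive facade color and detail brightness, and the roof material is swappable.
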(fn `UserConstructionScript`
  (bind _habillage_librairie (`self.Habillage_Librairie`))
  (bind _habillage_chapellerie (`self.Habillage_Chapellerie`))
  (bind _house (`self.House`))
  (bind _habillage_boucherie (`self.Habillage_Boucherie`))
  (bind _random_stream (`self.Random Stream`))
  (bind _rotation_volets_mid (`self.rotation volets mid`))
  (bind _rotation_volets_bas (`self.rotation volets bas`))
  (bind _rotation_volets_haut (`self.rotation volets haut`))
  (bind _voletbas1d (`self.voletBas1D`))
  (bind _fondations (`self.Fondations`))
  (bind _barriere5 (`self.Barriere5`))
  (`|ExecutionSequence`
    (:`then_0`
      ;[1 1 1] Visibility
      (if (`self.Volets?`)
        (`SceneComponent.SetVisibility` _voletbas1d true false)
        (`SceneComponent.SetVisibility` (`self.voletBas2D`) true false)
        (`SceneComponent.SetVisibility` (`self.voletBas1G`) true false)
        (`SceneComponent.SetVisibility` (`self.voletBas2G`) true false)
        (`SceneComponent.SetVisibility` (`self.voletMid2D`) true false)
        (`SceneComponent.SetVisibility` (`self.voletMid2G`) true false)
        (`SceneComponent.SetVisibility` (`self.voletMid1D`) true false)
        (`SceneComponent.SetVisibility` (`self.voletMid1G`) true false)
        (`SceneComponent.SetVisibility` (`self.voletHaut2G`) true false)
        (`SceneComponent.SetVisibility` (`self.voletHaut2D`) true false)
        (`SceneComponent.SetVisibility` (`self.voletHaut1G`) true false)
        (`SceneComponent.SetVisibility` (`self.voletHaut1D`) true false)
        (if (`self.RotRandom`)
          ;[1 1 1] Rotation Random
          (`|ExecutionSequence`
            (:`then_0`
              (set `self.rotation volets bas` (`KismetMathLibrary.SelectFloat` (`KismetMathLibrary.RandomFloatInRangeFromStream` 0.0 30.0 _random_stream) (`KismetMathLibrary.RandomFloatInRangeFromStream` 150.0 180.0 _random_stream) (`KismetMathLibrary.RandomBool`))))
            (:`then_1`
              (set `self.rotation volets mid` (`KismetMathLibrary.RandomFloatInRangeFromStream` 0.0 180.0 _random_stream)))
            (:`then_2`
              (set `self.rotation volets haut` (`KismetMathLibrary.RandomFloatInRangeFromStream` 30.0 180.0 _random_stream))
              ;[1 1 1] Rotation Variable
              (`|ExecutionSequence` :!label _label
                (:`then_0`
                  (`SceneComponent.K2_SetRelativeRotation` (`self.voletBas1D`) (`KismetMathLibrary.MakeRotator` 0.0 0.0 _rotation_volets_bas) false false)
                  (`SceneComponent.K2_SetRelativeRotation` (`self.voletBas2D`) (`KismetMathLibrary.MakeRotator` 0.0 0.0 _rotation_volets_bas) false false))
                (:`then_1`
                  (`SceneComponent.K2_SetRelativeRotation` (`self.voletBas1G`) (`KismetMathLibrary.MakeRotator` 0.0 0.0 (* _rotation_volets_bas -1.0)) false false)
                  (`SceneComponent.K2_SetRelativeRotation` (`self.voletBas2G`) (`KismetMathLibrary.MakeRotator` 0.0 0.0 (* _rotation_volets_bas -1.0)) false false))
                (:`then_2`
                  (`SceneComponent.K2_SetRelativeRotation` (`self.voletMid2D`) (`KismetMathLibrary.MakeRotator` 0.0 0.0 _rotation_volets_mid) false false)
                  (`SceneComponent.K2_SetRelativeRotation` (`self.voletMid1D`) (`KismetMathLibrary.MakeRotator` 0.0 0.0 _rotation_volets_mid) false false))
                (:`then_3`
                  (`SceneComponent.K2_SetRelativeRotation` (`self.voletMid2G`) (`KismetMathLibrary.MakeRotator` 0.0 0.0 (* _rotation_volets_mid -1.0)) false false)
                  (`SceneComponent.K2_SetRelativeRotation` (`self.voletMid1G`) (`KismetMathLibrary.MakeRotator` 0.0 0.0 (* _rotation_volets_mid -1.0)) false false))
                (:`then_4`
                  (`SceneComponent.K2_SetRelativeRotation` (`self.voletHaut2D`) (`KismetMathLibrary.MakeRotator` 0.0 0.0 _rotation_volets_haut) false false)
                  (`SceneComponent.K2_SetRelativeRotation` (`self.voletHaut1D`) (`KismetMathLibrary.MakeRotator` 0.0 0.0 _rotation_volets_haut) false false))
                (:`then_5`
                  (`SceneComponent.K2_SetRelativeRotation` (`self.voletHaut2G`) (`KismetMathLibrary.MakeRotator` 0.0 0.0 (* _rotation_volets_haut -1.0)) false false)
                  (`SceneComponent.K2_SetRelativeRotation` (`self.voletHaut1G`) (`KismetMathLibrary.MakeRotator` 0.0 0.0 (* _rotation_volets_haut -1.0)) false false)))))
          (else
            (goto _label)))
        (else
          (`SceneComponent.SetVisibility` _voletbas1d false false)
          (`SceneComponent.SetVisibility` (`self.voletBas2D`) false false)
          (`SceneComponent.SetVisibility` (`self.voletBas1G`) false false)
          (`SceneComponent.SetVisibility` (`self.voletBas2G`) false false)
          (`SceneComponent.SetVisibility` (`self.voletMid2D`) false false)
          (`SceneComponent.SetVisibility` (`self.voletMid2G`) false false)
          (`SceneComponent.SetVisibility` (`self.voletMid1D`) false false)
          (`SceneComponent.SetVisibility` (`self.voletMid1G`) false false)
          (`SceneComponent.SetVisibility` (`self.voletHaut2G`) false false)
          (`SceneComponent.SetVisibility` (`self.voletHaut2D`) false false)
          (`SceneComponent.SetVisibility` (`self.voletHaut1G`) false false)
          (`SceneComponent.SetVisibility` (`self.voletHaut1D`) false false))))
    (:`then_1`
      (if (`self.Fondation?`)
        (`SceneComponent.SetVisibility` _fondations true false)
        (else
          (`SceneComponent.SetVisibility` _fondations false false))))
    (:`then_2`
      (if (`self.Barrieres?`)
        (`SceneComponent.SetVisibility` _barriere5 true false)
        (`SceneComponent.SetVisibility` (`self.Barriere2`) true false)
        (`SceneComponent.SetVisibility` (`self.Barriere3`) true false)
        (`SceneComponent.SetVisibility` (`self.Barriere1`) true false)
        (else
          (`SceneComponent.SetVisibility` _barriere5 false false)
          (`SceneComponent.SetVisibility` (`self.Barriere2`) false false)
          (`SceneComponent.SetVisibility` (`self.Barriere3`) false false)
          (`SceneComponent.SetVisibility` (`self.Barriere1`) false false))))
    (:`then_3`
      (if (`self.Boucherie?`)
        (`SceneComponent.SetVisibility` _habillage_boucherie true false)
        (else
          (`SceneComponent.SetVisibility` _habillage_boucherie false false))))
    (:`then_4`
      (if (`self.Librairie?`)
        (`SceneComponent.SetVisibility` _habillage_librairie true false)
        (else
          (`SceneComponent.SetVisibility` _habillage_librairie false false))))
    (:`then_5`
      (if (`self.Chapellerie?`)
        (`SceneComponent.SetVisibility` _habillage_chapellerie true false)
        (else
          (`SceneComponent.SetVisibility` _habillage_chapellerie false false))))
    (:`then_6`
      ;[1 1 1] Color Control Facade
      (bind _returnvalue (`KismetMaterialLibrary.CreateDynamicMaterialInstance` "/Game/Environment_TA/Assets/Houses/Boutique02/Boutique02s/Boutique02_Vierge_+_Vitrine/Dossier_Materials/MI_Boutique02_Façadess.MI_Boutique02_Façadess"))
      (`MaterialInstanceDynamic.SetVectorParameterValue` _returnvalue "Color" (`self.Color Facade`))
      (`PrimitiveComponent.SetMaterial` (`self.House`) 2 _returnvalue)
      ;[1 1 1] Color Control Details
      (bind _returnvalue_2 (`KismetMaterialLibrary.CreateDynamicMaterialInstance` "/Game/Environment_TA/Assets/Houses/Boutique02/Boutique02s/Boutique02_Vierge_+_Vitrine/Dossier_Materials/MI_Boutique02_Détailss.MI_Boutique02_Détailss"))
      (`MaterialInstanceDynamic.SetScalarParameterValue` _returnvalue_2 "Color Intensity" (`self.Brightness Details`))
      (`PrimitiveComponent.SetMaterial` _house 1 _returnvalue_2)
      (`PrimitiveComponent.SetMaterial` _house 0 (`self.Roof Material`)))))
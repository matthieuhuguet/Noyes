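; BP_Underwater is an environment actor that sets up an underwater look from one set of exposed-style variables.
; The Construction Script pushes them into height fog with volumetric god rays, post process, skylight, sun with light function, and a bounce light.
; It also places a water surface plane with a dynamic material instance for color, metallic and opacity.
; Each component has its own visibility toggle, and no runtime logic runs.
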(fn `UserConstructionScript`
  (bind _exponentialheightfog (`self.ExponentialHeightFog`))
  (bind _postprocess (`self.PostProcess`))
  (bind _skylight (`self.SkyLight`))
  (bind _directionallight (`self.DirectionalLight`))
  (bind _plane_surface (`self.Plane_Surface`))
  (bind _sunlight_bounced (`self.SunLight Bounced`))
  (bind (_saturation _contrast _gamma _gain _offset) (break `ColorGradePerRangeSettings` (`self.Color Grade Settings`)))
  ;[0.1278 0.25 0.1073] Fog
  (`SceneComponent.SetVisibility` _exponentialheightfog (`self.Fog Visibility`) false)
  (`ExponentialHeightFogComponent.SetStartDistance` _exponentialheightfog (`self.Fog Distance`))
  (`ExponentialHeightFogComponent.SetDirectionalInscatteringExponent` _exponentialheightfog (`self.Top surface scattering`))
  (`ExponentialHeightFogComponent.SetFogMaxOpacity` _exponentialheightfog (`self.Fog Opacity`))
  (`ExponentialHeightFogComponent.SetFogInscatteringColor` _exponentialheightfog (`self.Fog Color`))
  (`ExponentialHeightFogComponent.SetDirectionalInscatteringColor` _exponentialheightfog (`self.Top Surface Color`))
  (`ExponentialHeightFogComponent.SetVolumetricFog` _exponentialheightfog (`self.Volumetric Fog (GodRays)`))
  (`ExponentialHeightFogComponent.SetVolumetricFogScatteringDistribution` _exponentialheightfog (`self.God Rays Qté`))
  (`ExponentialHeightFogComponent.SetVolumetricFogExtinctionScale` _exponentialheightfog (`self.God Rays Scale`))
  (`ExponentialHeightFogComponent.SetVolumetricFogAlbedo` _exponentialheightfog (`self.Volumetric Albedo`))
  (`ExponentialHeightFogComponent.SetVolumetricFogDistance` _exponentialheightfog (`self.Volumetric Distance`))
  (`ExponentialHeightFogComponent.SetVolumetricFogEmissive` _exponentialheightfog (`self.God Rays Emissive`))
  ;[0.7648 0.4856 0.8125] Post process
  (`SceneComponent.SetVisibility` _postprocess (`self.Post process Visibility`) false)
  (setmembers `PostProcessSettings` :`StructRef` (`PostProcessComponent.Settings` _postprocess) :`BloomMethod` "BM_FFT" :`WhiteTemp` (`self.Temp`) :`WhiteTint` (`self.Tint`) :`ColorSaturation` _saturation :`ColorContrast` _contrast :`ColorGamma` _gamma :`ColorGain` _gain :`ColorOffset` _offset :`SceneFringeIntensity` (`self.Chromatic Intensity`) :`BloomIntensity` (`self.Water Blur`) :`DynamicGlobalIlluminationMethod` "Lumen" :`ReflectionMethod` "Lumen" :`AutoExposureBias` (`self.Exposure`) :`VignetteIntensity` (`self.Vignette Intensity`) :`WeightedBlendables` (`self.Post Process Materials`))
  ;[0.9073 1 0.552] Skylight
  (`SceneComponent.SetVisibility` _skylight (`self.Skylight Visibility`) false)
  (`SkyLightComponent.SetIntensity` _skylight (`self.Skylight Intensity`))
  (`SkyLightComponent.SetCubemap` _skylight (`self.Cubemap`))
  (`SkyLightComponent.SetLightColor` _skylight (`self.Skylight Tint Color`))
  ;[1 0.6816 0.5086] Sun Light
  (`SceneComponent.SetVisibility` _directionallight (`self.Sun Light Visibility`) false)
  (`LightComponent.SetIntensity` _directionallight (`self.Sun Light Intensity`))
  (`LightComponent.SetLightColor` _directionallight (`self.Sun Light Color`) true)
  (`DirectionalLightComponent.SetLightSourceSoftAngle` _directionallight (`self.Sun Light Soft Shadow`))
  (`LightComponent.SetLightFunctionMaterial` _directionallight (`self.Light Function Material`))
  (`LightComponent.SetLightFunctionScale` _directionallight (`self.Light Function Scale`))
  (`LightComponent.SetVolumetricScatteringIntensity` _directionallight (`self.Volumetric Light`))
  (`LightComponentBase.SetCastVolumetricShadow` _directionallight (`self.Volumetric Shadows`))
  (`SceneComponent.K2_SetWorldTransform` _directionallight (`self.Sun Light Transform`) false false)
  ;[0.396 0.4194 1] Surface Plane
  (`SceneComponent.SetVisibility` _plane_surface (`self.Surface Plane Visibility`) false)
  (`SceneComponent.K2_SetWorldTransform` _plane_surface (`self.Surface Transform`) false false)
  (bind _returnvalue (`KismetMaterialLibrary.CreateDynamicMaterialInstance` (`self.Surface Material`)))
  (`MaterialInstanceDynamic.SetVectorParameterValue` _returnvalue "subsurface" (`self.Surface Color`))
  (`MaterialInstanceDynamic.SetScalarParameterValue` _returnvalue "metallic" (`self.Metallic`))
  (`MaterialInstanceDynamic.SetScalarParameterValue` _returnvalue "opacity" (`self.Opacity`))
  (`PrimitiveComponent.SetMaterial` _plane_surface 0 _returnvalue)
  ;[1 1 1] Bounce Light
  (`SceneComponent.SetVisibility` _sunlight_bounced (`self.Bounce Light Visibility`) false)
  (`LightComponent.SetLightColor` _sunlight_bounced (`self.Bounce Light Color`) true)
  (`LightComponent.SetIntensity` _sunlight_bounced (`self.Bounce Light Intensity`)))
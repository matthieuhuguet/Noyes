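; BP_Barrieres is an environment utility that builds a row of barriers along an editable spline.
; Its construction script divides the spline by a segment length and adds a spline mesh per segment, randomly picked from three options, with tangents clamped to that length.
; It also places a static mesh at each segment start, aligned to the spline.
; Nodes for disabling collision and alternating material color are left disconnected.
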(fn `UserConstructionScript`
  (bind _spline (`self.Spline`))
  (for _index (range (`KismetMathLibrary.FTrunc` (/ (`SplineComponent.GetSplineLength` (`self.Spline`)) (`self.Lenght`))))
    (bind _returnvalue (`AddComponent|NODE_AddSplineMeshComponent-0`))
    (`StaticMeshComponent.SetStaticMesh` _returnvalue (select `int` (`KismetMathLibrary.RandomIntegerInRange` 0 2) :`0` (`self.Option 0`) :`1` (`self.Option 1`) :`2` (`self.Option 2`)))
    (`SplineMeshComponent.SetForwardAxis` _returnvalue "X" true)
    (bind _returnvalue_2 (* _index (`self.Lenght`)))
    (bind _returnvalue_3 (`SplineComponent.GetLocationAtDistanceAlongSpline` _spline _returnvalue_2 "Local"))
    (bind _returnvalue_4 (* (+ _index 1) (`self.Lenght`)))
    (`SplineMeshComponent.SetStartAndEnd` _returnvalue _returnvalue_3 (`KismetMathLibrary.ClampVectorSize` (`SplineComponent.GetTangentAtDistanceAlongSpline` _spline _returnvalue_2 "Local") 0.0 (`self.Lenght`)) (`SplineComponent.GetLocationAtDistanceAlongSpline` _spline _returnvalue_4 "Local") (`KismetMathLibrary.ClampVectorSize` (`SplineComponent.GetTangentAtDistanceAlongSpline` _spline _returnvalue_4 "Local") 0.0 (`self.Lenght`)) true)
    (`AddComponent|NODE_AddStaticMeshComponent-4` :`RelativeTransform` (`KismetMathLibrary.MakeTransform` _returnvalue_3 (`SplineComponent.GetRotationAtDistanceAlongSpline` _spline (* _index (`self.Lenght`)) "Local")))))
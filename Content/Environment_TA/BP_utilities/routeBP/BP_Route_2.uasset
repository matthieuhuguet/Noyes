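; Route utility actor that builds a mesh along a spline in its construction script, with collision enabled.
; It adds spline mesh components using SelectMesh at OffsetAdjust intervals, with roll taken from the spline.
; Tangents are length-clamped to the interval, though StartTangent receives the next location and EndPos a clamped tangent.
; Per-point loops, one gated by Egouts, are unconnected, and the event graph is empty.
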(fn `UserConstructionScript`
  (bind _offset_adjust (`self.Offset adjust`))
  (bind _offset_adjust_2 (`self.Offset adjust`))
  (bind _spline (`self.Spline`))
  (bind _spline_2 (`self.Spline`))
  (`|ExecutionSequence`
    (:`then_0`
      (for _index (range (+ (`KismetMathLibrary.FTrunc` (/ (`SplineComponent.GetSplineLength` (`self.Spline`)) (`self.Offset adjust`))) 1))
        (bind _returnvalue (`AddComponent|NODE_AddSplineMeshComponent-6`))
        (`StaticMeshComponent.SetStaticMesh` _returnvalue (`self.Select mesh`))
        (`PrimitiveComponent.SetCollisionEnabled` _returnvalue "QueryAndPhysics")
        (bind _returnvalue_2 (* _index _offset_adjust_2))
        (bind _returnvalue_3 (* _offset_adjust_2 (+ _index 1)))
        (`SplineMeshComponent.SetStartAndEnd` _returnvalue (`SplineComponent.GetLocationAtDistanceAlongSpline` _spline _returnvalue_2 "Local") (`SplineComponent.GetLocationAtDistanceAlongSpline` _spline _returnvalue_3 "Local") (`KismetMathLibrary.ClampVectorSize` (`SplineComponent.GetTangentAtDistanceAlongSpline` _spline _returnvalue_2 "Local") 0.0 _offset_adjust) (`KismetMathLibrary.ClampVectorSize` (`SplineComponent.GetTangentAtDistanceAlongSpline` _spline _returnvalue_3 "Local") 0.0 _offset_adjust) true)
        (bind _returnvalue_roll (`KismetMathLibrary.BreakRotator` (`SplineComponent.GetRotationAtDistanceAlongSpline` _spline_2 _returnvalue_2 "Local")))
        (`SplineMeshComponent.SetStartRoll` _returnvalue _returnvalue_roll true)
        (bind _returnvalue_roll_2 (`KismetMathLibrary.BreakRotator` (`SplineComponent.GetRotationAtDistanceAlongSpline` _spline_2 _returnvalue_3 "Local")))
        (`SplineMeshComponent.SetEndRoll` _returnvalue _returnvalue_roll_2 true)))))
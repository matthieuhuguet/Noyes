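; BP_Canard is a destructible duck actor in a personal test folder.
; Any damage it takes is subtracted from its health variable, VieCanard, which is clamped so it cannot drop below zero.
; When health reaches zero, it destroys itself, then spawns an explosion emitter at its location and plays a 2D toy duck sound.
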(event `self.ReceiveAnyDamage`
  (params (Damage :type "Float (single-precision)") (DamageType :type "DamageType Object Reference") (InstigatedBy :type "Controller Object Reference") (DamageCauser :type "Actor Object Reference"))
  (set `self.VieCanard` (`KismetMathLibrary.FClamp` (- (`self.VieCanard`) Damage) 0.0 (`self.VieCanard`)))
  (if (== (`self.VieCanard`) 0.0)
    (`self.K2_DestroyActor`)
    (`GameplayStatics.SpawnEmitterAtLocation` "/Game/Environment_TA/StarterContent/Particles/P_Explosion.P_Explosion" (`self.K2_GetActorLocation`))
    (`GameplayStatics.PlaySound2D` "/Game/Environment_TA/Personal/Enzo/Test_Eglise/Canard/toy_duck_sound.toy_duck_sound" 1.0 1.0 0.0 null null)))

(fn `UserConstructionScript`)